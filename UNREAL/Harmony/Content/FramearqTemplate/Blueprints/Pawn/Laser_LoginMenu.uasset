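; Laser pointer actor for the login menu that draws a beam from the login pawn's camera, or a supplied start location, toward a hit point.
; Each tick it computes beam endpoints from a supplied or cursor/touch hit, then passes them through UpdateOnServer.
; SetLaserMesh orients and stretches the beam and places a distance-scaled sphere at the end.
; BeginPlay applies the laser color to both meshes.
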(event Custom|SetLaserMesh
  (params (End :type Vector) (Start :type Vector))
  (bind _returnvalue (- End Start))
  (bind _worldscale (Variables|Default|GetWorldScale))
  (bind _sphere (Variables|Default|GetSphere))
  (bind _laserscaleroot (Variables|Default|GetLaserScaleRoot))
  (bind _returnvalue_2 (Math|Vector|VectorLength _returnvalue))
  (bind _returnvalue_3 (* 0.004 _worldscale))
  (bind _returnvalue_4 (Math|Float|NormalizetoRange _returnvalue_2 -1e+02 4e+02))
  (bind _returnvalue_5 (* _returnvalue_4 0.05))
  (bind _returnvalue_6 (Math|Float|Absolute(Float) _returnvalue_5))
  ;[0.2555 0.7775 1] updateLaserEvent
  (Transformation|SetWorldLocation _laserscaleroot Start false false)
  (Transformation|SetWorldRotation _laserscaleroot (Math|Rotator|MakeRotfromZ _returnvalue) false false)
  (Transformation|SetWorldScale3D (Variables|Default|GetLaserScaleRoot) (Math|Vector|MakeVector _returnvalue_3 _returnvalue_3 (* _returnvalue_2 0.01)))
  (Transformation|SetWorldLocation _sphere End false false)
  (Transformation|SetWorldScale3D _sphere (Math|Vector|MakeVector _returnvalue_6 _returnvalue_6 _returnvalue_6)))

(event Custom|UpdateLaser
  (params (OffsetStartLocation :type Vector) (StartLocation :type Vector) (SetStartLocation :type Boolean) (hit :type Hit%20Result%20Structure))
  ;[0.2555 0.7775 1] updateLaserEvent
  (CallFunction|GetLaserLocations (select SetStartLocation hit (|MakeTouchAndMouseHit_2)) OffsetStartLocation StartLocation SetStartLocation))

(event Custom|UpdateOnServer
  (params (HitLaserStart :type Vector) (HitLaserEnd :type Vector))
  ;[0.2555 0.7775 1] updateLaserEvent
  (Variables|Default|SetHitLaserStart HitLaserStart)
  (Variables|Default|SetHitLaserEnd HitLaserEnd))

(event EventBeginPlay
  (CallFunction|ChangeColors (Utilities|Array|MakeArray (Variables|Default|GetSphere) (Variables|Default|GetLaserMesh)) (Variables|Default|GetColor)))

(event EventTick
  (params (DeltaSeconds :type Float%20%28single-precision%29))
  (CallFunction|UpdateLaser (Variables|Default|GetOffsetStartLocation) (Variables|Default|GetStartLocation) (Variables|Default|GetSetStartLocation) (Variables|Default|GetHit))
  (CallFunction|UpdateonServer (Variables|Default|GetHitLaserStart) (Variables|Default|GetHitLaserEnd))
  (CallFunction|SetLaserMesh (Variables|Default|GetHitLaserEnd) (Variables|Default|GetHitLaserStart)))

(fn ConstructionScript)

(fn GetLaserLocations
  (params (Hit :type Hit%20Result%20Structure%20%28by%20ref%29) (OffsetStartLocation_ :type Vector) (StartLocation_ :type Vector) (SetStartLocation_ :type Boolean))
  (bind _returnvalue (Game|Player|GetPlayerPawn 0))
  (bind (_bblockinghit _binitialoverlap _time _distance _location) (Collision|BreakHitResult Hit))
  (bind _asbp_login_menu_pawn_final (Utilities|Casting|CastToBP_LoginMenu_PawnFinal _returnvalue))
  (bind _camera (Variables|/Game/FramearqTemplate/Blueprints/Pawn/BP_LoginMenu_PawnFinal.BP_LoginMenu_PawnFinal_C|GetCamera _asbp_login_menu_pawn_final))
  (bind _returnvalue_2 (Transformation|GetWorldLocation _camera))
  (bind _returnvalue_3 (select SetStartLocation_ StartLocation_ _returnvalue_2))
  (bind _returnvalue_4 (+ _returnvalue_3 OffsetStartLocation_))
  (Variables|Default|SetHitLaserStart _returnvalue_4)
  (Variables|Default|SetHitLaserEnd (select _bblockinghit _location _returnvalue_4)))

(fn OnRepColor)