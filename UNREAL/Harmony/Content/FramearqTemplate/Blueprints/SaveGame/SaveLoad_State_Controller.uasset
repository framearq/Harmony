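; Player controller component that manages named save states for desktop and VR menus in a collaborative template.
; On startup it loads or creates the MainSaveGame name index and default state slot, then fills the persistent UI's state list.
; It binds save and load events on that UI and the VR pawn's toolbar, and passes requests to the pawn's SaveLoad_State_Pawn component.
; Initial index registration runs through ROS/MTC events, writing only on non-dedicated-server instances.
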(event Custom|MainSaveGameToPersistentMenu
  (bind _returnvalue (Game|GetPlayerController 0))
  (bind _asbp_collab_v_player_controller (Utilities|Casting|CastToBP_Collab_V_PlayerController _returnvalue))
  (bind _persistent_ui (Variables|/Game/FramearqTemplate/Blueprints/PlayerController/BP_Collab_V_PlayerController.BP_Collab_V_PlayerController_C|GetPersistent_UI _asbp_collab_v_player_controller))
  (Utilities|IsValid _persistent_ui
    (:Is%20Valid
      (for _array_element (Variables|/Game/FramearqTemplate/Blueprints/SaveGame/BP_Name_SaveGame.BP_Name_SaveGame_C|GetSaveGameNameArray (Variables|Default|GetSaveGame))
        (Default|AddOption (Variables|/Game/FramearqTemplate/UMG/GameMenu/Persistent_ToolBar.Persistent_ToolBar_C|GetLoadStateComboBox _persistent_ui) _array_element)))))

(event Custom|CreateMainSlot_SaveGame
  (bind _default_state_name (Variables|Default|GetDefault_state_name))
  (if (Class|BlueprintPathsLibrary|FileExists (Utilities|String|Append (Class|KismetSystemLibrary|GetProjectSavedDirectory) "SaveGames/MainSaveGame.sav"))
    (bind _returnvalue (SaveGame|LoadGamefromSlot "MainSaveGame"))
    (bind _asbp_name_save_game (Utilities|Casting|CastToBP_Name_SaveGame _returnvalue))
    (Variables|Default|SetSaveGame _asbp_name_save_game)
    (else
      (bind _returnvalue_2 (SaveGame|CreateSaveGameObject "/Game/FramearqTemplate/Blueprints/SaveGame/BP_Name_SaveGame.BP_Name_SaveGame_C"))
      (Variables|Default|SetSaveGame _returnvalue_2)
      (bind _returnvalue_3 (SaveGame|CreateSaveGameObject "/Game/FramearqTemplate/Blueprints/SaveGame/BP_Data_SaveGame.BP_Data_SaveGame_C"))
      (SaveGame|SaveGametoSlot _returnvalue_3 _default_state_name)
      (CallFunction|CreateIntialSaveGameROS _default_state_name)))
  (Utilities|FlowControl|Sequence
    (:then_0
      (Default|SetSelectedOption (Variables|/Game/FramearqTemplate/UMG/GameMenu/Persistent_ToolBar.Persistent_ToolBar_C|GetLoadStateComboBox (Variables|Default|GetPersistent_UI)) _default_state_name))
    (:then_1
      (bind _asbp_vrpawn (Utilities|Casting|CastToBP_VRPawn (Game|Player|GetPlayerPawn 0)))
      (Utilities|IsValid _asbp_vrpawn
        (:Is%20Valid
          (bind _aspersistent_tool_bar (Utilities|Casting|CastToPersistent_ToolBar (UserInterface|GetWidget (Variables|/Game/FramearqTemplate/Blueprints/Pawn/VR/BP_VRPawn.BP_VRPawn_C|GetPersistentToolBar_VR _asbp_vrpawn))))
          (Default|SetSelectedOption (Variables|/Game/FramearqTemplate/UMG/GameMenu/Persistent_ToolBar.Persistent_ToolBar_C|GetLoadStateComboBox _aspersistent_tool_bar) _default_state_name))))))

(event Custom|AddToMainSveGame
  (params (SlotName :type String%20%28by%20ref%29))
  (Default|SaveGameROS (Actor|GetComponentbyClass (Game|Player|GetPlayerPawn 0) "/Game/FramearqTemplate/Blueprints/SaveGame/SaveLoad_State_Pawn.SaveLoad_State_Pawn_C") SlotName (Variables|Default|GetSaveGame)))

(event Custom|BindToMenu
  (Utilities|FlowControl|Sequence
    (:then_0
      ;[1 0 0] save new slot in vr
      (bind _asbp_vrpawn (Utilities|Casting|CastToBP_VRPawn (Game|Player|GetPlayerPawn 0)))
      (Utilities|IsValid _asbp_vrpawn
        (:Is%20Valid
          (bind _aspersistent_tool_bar (Utilities|Casting|CastToPersistent_ToolBar (UserInterface|GetWidget (Variables|/Game/FramearqTemplate/Blueprints/Pawn/VR/BP_VRPawn.BP_VRPawn_C|GetPersistentToolBar_VR _asbp_vrpawn))))
          (EventDispatchers|BindEventtoSavingState _aspersistent_tool_bar (EventDispatchers|CreateEvent :!event Custom|AddToMainSveGame))
          (EventDispatchers|BindEventtoLoadState _aspersistent_tool_bar (EventDispatchers|CreateEvent :!event Custom|LoadSaveGame)))))
    (:then_1
      (bind _asbp_collab_v_player_controller (Utilities|Casting|CastToBP_Collab_V_PlayerController (Game|GetPlayerController 0)))
      (EventDispatchers|BindEventtoSavingState (Variables|/Game/FramearqTemplate/Blueprints/PlayerController/BP_Collab_V_PlayerController.BP_Collab_V_PlayerController_C|GetPersistent_UI _asbp_collab_v_player_controller) (EventDispatchers|CreateEvent :!event Custom|AddToMainSveGame))
      (EventDispatchers|BindEventtoLoadState (Variables|/Game/FramearqTemplate/Blueprints/PlayerController/BP_Collab_V_PlayerController.BP_Collab_V_PlayerController_C|GetPersistent_UI _asbp_collab_v_player_controller) (EventDispatchers|CreateEvent :!event Custom|LoadSaveGame)))))

(event Custom|BeginPlayFromController
  (Utilities|FlowControl|DoOnce false
    (:Completed
      (bind _asbp_collab_v_player_controller (Utilities|Casting|CastToBP_Collab_V_PlayerController (Game|GetPlayerController 0)))
      (Variables|Default|SetPersistent_UI (Variables|/Game/FramearqTemplate/Blueprints/PlayerController/BP_Collab_V_PlayerController.BP_Collab_V_PlayerController_C|GetPersistent_UI _asbp_collab_v_player_controller))
      (CallFunction|CreateMainSlotSaveGame)
      (CallFunction|MainSaveGametoPersistentMenu)
      (CallFunction|BindtoMenu))))

(event Custom|Create%20intial%20save%20Game%20ROS
  (params (Default%20initial%20state%20name :type String))
  (CallFunction|CreateInitialSaveGameMTC Default%20initial%20state%20name))

(event Custom|Create%20initial%20save%20Game%20MTC
  (params (Default%20initial%20state%20name :type String))
  (if (not (Networking|IsDedicatedServer))
    (bind _asbp_collab_v_player_controller (Utilities|Casting|CastToBP_Collab_V_PlayerController (Game|GetPlayerController 0)))
    (Utilities|Array|Add (Variables|/Game/FramearqTemplate/Blueprints/SaveGame/BP_Name_SaveGame.BP_Name_SaveGame_C|GetSaveGameNameArray (Variables|SaveLoad_State_Controller_C|GetSaveGame (Variables|/Game/FramearqTemplate/Blueprints/PlayerController/BP_Collab_V_PlayerController.BP_Collab_V_PlayerController_C|GetSaveLoad_State_Controller _asbp_collab_v_player_controller))) Default%20initial%20state%20name)
    (Utilities|IsValid (Variables|SaveLoad_State_Controller_C|GetSaveGame (Variables|/Game/FramearqTemplate/Blueprints/PlayerController/BP_Collab_V_PlayerController.BP_Collab_V_PlayerController_C|GetSaveLoad_State_Controller _asbp_collab_v_player_controller))
      (:Is%20Valid
        (SaveGame|SaveGametoSlot (Variables|SaveLoad_State_Controller_C|GetSaveGame (Variables|/Game/FramearqTemplate/Blueprints/PlayerController/BP_Collab_V_PlayerController.BP_Collab_V_PlayerController_C|GetSaveLoad_State_Controller _asbp_collab_v_player_controller)) "MainSaveGame")))))

(event Custom|LoadSaveGame
  (params (Option :type String) (SaveGameMain :type BP%20Data%20Save%20Game%20Object%20Reference))
  (Default|LoadSaveGameROS (Actor|GetComponentbyClass (Game|Player|GetPlayerPawn 0) "/Game/FramearqTemplate/Blueprints/SaveGame/SaveLoad_State_Pawn.SaveLoad_State_Pawn_C") Option SaveGameMain))

(fn HMDState
  (return (Math|Boolean|ORBoolean (Class|HeadMountedDisplayFunctionLibrary|IsHeadMountedDisplayEnabled) (and (Utilities|Enum|Equal(Enum) (Game|GetPlatformName) "Android") (Utilities|Name|NotEqual(Name) (Class|HeadMountedDisplayFunctionLibrary|GetHMDDeviceName) "None")) (== (Class|HeadMountedDisplayFunctionLibrary|GetHMDWornState) 1))))