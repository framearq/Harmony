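; Save/load state Blueprint that keeps the saved-state list and toolbar selection in step, with events named as server-to-multicast (ROS/MTC) pairs.
; Saving adds the name to the VR pawn's toolbar or desktop PersistentUI, depending on headset checks, and writes it to "MainSaveGame", skipping dedicated servers.
; Loading only updates the combo box selection in both UIs.
; Clearing empties the player controller's DataSaveGame arrays.
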(event Custom|LoadSaveGameMTC
  (params (Option :type String))
  (Utilities|FlowControl|Sequence
    (:then_0
      (bind _asbp_vrpawn (Utilities|Casting|CastToBP_VRPawn (Game|Player|GetPlayerPawn 0)))
      (Utilities|IsValid _asbp_vrpawn
        (:Is%20Valid
          (bind _aspersistent_tool_bar (Utilities|Casting|CastToPersistent_ToolBar (UserInterface|GetWidget (Variables|/Game/FramearqTemplate/Blueprints/Pawn/VR/BP_VRPawn.BP_VRPawn_C|GetPersistentToolBar_VR _asbp_vrpawn))))
          (Default|SetSelectedOption (Variables|/Game/FramearqTemplate/UMG/GameMenu/Persistent_ToolBar.Persistent_ToolBar_C|GetLoadStateComboBox _aspersistent_tool_bar) Option))))
    (:then_1
      (bind _persistent_ui (Variables|Default|GetPersistent_UI)
        (:then
          (Default|SetSelectedOption (Variables|/Game/FramearqTemplate/UMG/GameMenu/Persistent_ToolBar.Persistent_ToolBar_C|GetLoadStateComboBox _persistent_ui) Option))
        (:else)))))

(event Custom|SaveGameMTC
  (params (Option :type String) (SaveGame :type BP%20Name%20Save%20Game%20Object%20Reference))
  (bind _persistent_ui (Variables|Default|GetPersistent_UI))
  (bind _loadstatecombobox (Variables|/Game/FramearqTemplate/UMG/GameMenu/Persistent_ToolBar.Persistent_ToolBar_C|GetLoadStateComboBox _persistent_ui))
  (if (not (Networking|IsDedicatedServer))
    (if (Math|Boolean|ORBoolean (Class|HeadMountedDisplayFunctionLibrary|IsHeadMountedDisplayEnabled) (and (Utilities|Enum|Equal(Enum) (Game|GetPlatformName) "Android") (Utilities|Name|NotEqual(Name) (Class|HeadMountedDisplayFunctionLibrary|GetHMDDeviceName) "None")) (== (Class|HeadMountedDisplayFunctionLibrary|GetHMDWornState) 1))
      ;[1 0 0] test
      (bind _asbp_vrpawn (Utilities|Casting|CastToBP_VRPawn (Game|Player|GetPlayerPawn 0)))
      (Utilities|IsValid _asbp_vrpawn
        (:Is%20Valid
          (bind _aspersistent_tool_bar (Utilities|Casting|CastToPersistent_ToolBar (UserInterface|GetWidget (Variables|/Game/FramearqTemplate/Blueprints/Pawn/VR/BP_VRPawn.BP_VRPawn_C|GetPersistentToolBar_VR _asbp_vrpawn))))
          (Default|AddOption (Variables|/Game/FramearqTemplate/UMG/GameMenu/Persistent_ToolBar.Persistent_ToolBar_C|GetLoadStateComboBox _aspersistent_tool_bar) Option)
          (Default|SetSelectedOption (Variables|/Game/FramearqTemplate/UMG/GameMenu/Persistent_ToolBar.Persistent_ToolBar_C|GetLoadStateComboBox _aspersistent_tool_bar) Option)
          (bind _asbp_collab_v_player_controller (Utilities|Casting|CastToBP_Collab_V_PlayerController (Game|GetPlayerController 0)))
          (Utilities|Array|Add (Variables|/Game/FramearqTemplate/Blueprints/SaveGame/BP_Name_SaveGame.BP_Name_SaveGame_C|GetSaveGameNameArray (Variables|/Game/FramearqTemplate/Blueprints/SaveGame/SaveLoad_State_Controller.SaveLoad_State_Controller_C|GetSaveGame (Variables|/Game/FramearqTemplate/Blueprints/PlayerController/BP_Collab_V_PlayerController.BP_Collab_V_PlayerController_C|GetSaveLoad_State_Controller _asbp_collab_v_player_controller))) Option)
          (Utilities|IsValid (Variables|/Game/FramearqTemplate/Blueprints/SaveGame/SaveLoad_State_Controller.SaveLoad_State_Controller_C|GetSaveGame (Variables|/Game/FramearqTemplate/Blueprints/PlayerController/BP_Collab_V_PlayerController.BP_Collab_V_PlayerController_C|GetSaveLoad_State_Controller _asbp_collab_v_player_controller))
            (:Is%20Valid
              (SaveGame|SaveGametoSlot (Variables|/Game/FramearqTemplate/Blueprints/SaveGame/SaveLoad_State_Controller.SaveLoad_State_Controller_C|GetSaveGame (Variables|/Game/FramearqTemplate/Blueprints/PlayerController/BP_Collab_V_PlayerController.BP_Collab_V_PlayerController_C|GetSaveLoad_State_Controller _asbp_collab_v_player_controller)) "MainSaveGame")))))
      (else
        (bind _asbp_collab_v_player_controller_2 (Utilities|Casting|CastToBP_Collab_V_PlayerController (Game|GetPlayerController 0)))
        (Default|AddOption _loadstatecombobox Option)
        (Default|SetSelectedOption _loadstatecombobox Option)
        (Utilities|Array|Add (Variables|/Game/FramearqTemplate/Blueprints/SaveGame/BP_Name_SaveGame.BP_Name_SaveGame_C|GetSaveGameNameArray (Variables|/Game/FramearqTemplate/Blueprints/SaveGame/SaveLoad_State_Controller.SaveLoad_State_Controller_C|GetSaveGame (Variables|/Game/FramearqTemplate/Blueprints/PlayerController/BP_Collab_V_PlayerController.BP_Collab_V_PlayerController_C|GetSaveLoad_State_Controller _asbp_collab_v_player_controller_2))) Option)
        (Utilities|IsValid (Variables|/Game/FramearqTemplate/Blueprints/SaveGame/SaveLoad_State_Controller.SaveLoad_State_Controller_C|GetSaveGame (Variables|/Game/FramearqTemplate/Blueprints/PlayerController/BP_Collab_V_PlayerController.BP_Collab_V_PlayerController_C|GetSaveLoad_State_Controller _asbp_collab_v_player_controller_2))
          (:Is%20Valid
            (SaveGame|SaveGametoSlot (Variables|/Game/FramearqTemplate/Blueprints/SaveGame/SaveLoad_State_Controller.SaveLoad_State_Controller_C|GetSaveGame (Variables|/Game/FramearqTemplate/Blueprints/PlayerController/BP_Collab_V_PlayerController.BP_Collab_V_PlayerController_C|GetSaveLoad_State_Controller _asbp_collab_v_player_controller_2)) "MainSaveGame")))))))

(event Custom|LoadSaveGameROS
  (params (Option :type String) (SaveGame :type BP%20Data%20Save%20Game%20Object%20Reference))
  (CallFunction|LoadSaveGameMTC Option))

(event Custom|ClearSaveGamesArraysROS
  (CallFunction|ClearSaveGamesArraysMTC))

(event Custom|ClearSaveGamesArraysMTC
  (bind _asbp_collab_v_player_controller (Utilities|Casting|CastToBP_Collab_V_PlayerController (Game|GetPlayerController 0)))
  (Default|ClearSaveGameArrays (Variables|/Game/FramearqTemplate/Blueprints/PlayerController/BP_Collab_V_PlayerController.BP_Collab_V_PlayerController_C|GetDataSaveGame _asbp_collab_v_player_controller)))

(event Custom|SaveGameROS
  (params (Option :type String) (SaveGame :type BP%20Name%20Save%20Game%20Object%20Reference))
  (CallFunction|SaveGameMTC Option SaveGame))

(event EventBeginPlay
  (bind _asbp_collab_v_player_controller (Utilities|Casting|CastToBP_Collab_V_PlayerController (Game|GetPlayerController 0)))
  (Variables|Default|SetPersistent_UI (Variables|/Game/FramearqTemplate/Blueprints/PlayerController/BP_Collab_V_PlayerController.BP_Collab_V_PlayerController_C|GetPersistent_UI _asbp_collab_v_player_controller)))