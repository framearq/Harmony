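; BP_PickupObject is a physics prop that VR motion controllers can pick up and drop, with up to two constraints holding it at once.
; Pickup binds the hand to the static mesh through the passed constraint and turns off actor, movement and mesh replication.
; Drop re-enables replication, even if another grip remains, then breaks the matching constraint, promoting the second to first when needed.
; The construction script overrides mesh mass from KG.
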(event EventBeginPlay)

(event Collision|EventActorBeginOverlap
  (params (OtherActor :type Actor%20Object%20Reference)))

(event EventPickup
  (params (AttachTo :type Scene%20Component%20Object%20Reference) (Constraint :type Physics%20Constraint%20Component%20Object%20Reference) (Hand :type Skeletal%20Mesh%20Component%20Object%20Reference))
  ;[1 1 1] Pickup
  (Networking|SetReplicates false)
  (Class|Actor|SetReplicateMovement false)
  (Class|ActorComponent|SetIsReplicated (Variables|Debug|GetStaticMeshComponent) false)
  (Class|PhysicsConstraintComponent|SetConstrainedComponents Constraint Hand "None" (Variables|Debug|GetStaticMeshComponent) "None")
  (Variables|Default|GetConstraint1
    (:then
      (Variables|Default|SetConstraint2 Constraint))
    (:else
      (Variables|Default|SetConstraint1 Constraint))))

(event EventDrop
  (params (Constraint :type Physics%20Constraint%20Component%20Object%20Reference))
  ;[1 1 1] Drop
  (Networking|SetReplicates true)
  (Class|Actor|SetReplicateMovement true)
  (Class|ActorComponent|SetIsReplicated (Variables|Debug|GetStaticMeshComponent) true)
  (bind _constraint1 (Variables|Default|GetConstraint1)
    (:then
      (if (== _constraint1 Constraint)
        (Class|PhysicsConstraintComponent|BreakConstraint (Variables|Default|GetConstraint1))
        (Variables|Default|SetConstraint1 0)
        (bind _constraint2 (Variables|Default|GetConstraint2)
          (:then
            (Variables|Default|SetConstraint1 _constraint2)
            (Variables|Default|SetConstraint2 0))
          (:else))
        (else
          (bind _constraint2_2 (Variables|Default|GetConstraint2)
            (:then
              (if (== _constraint2_2 Constraint)
                (Class|PhysicsConstraintComponent|BreakConstraint (Variables|Default|GetConstraint2))
                (Variables|Default|SetConstraint2 0)))
            (:else)))))
    (:else)))

(fn ConstructionScript
  (Class|PrimitiveComponent|SetMassOverrideinKg (Variables|Debug|GetStaticMeshComponent) "None" (Variables|Default|GetKG) true))