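; Snapshot command for the Framearq template that, on Windows only, adds a contextual "Instantánea" button with a take-photo option.
; Enabling it narrows the pawn's object types and replaces any BP_Photo with a new frame at the camera, scaled to world scale.
; The option calls DoCapture on that frame; disabling restores object types and FOV, resets BP_TransformComponent and destroys the frame.
; The left-mouse handler is empty, leaving the frame-transform logic unconnected.
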(event Custom|Enabled
  (bind _basepawn (Variables|Default|GetBasePawn))
  ;[0.3384 0.6313 1] Setup Option Buttons
  (Variables|Default|SetActivated true)
  (Variables|/Game/FramearqTemplate/Blueprints/Pawn/BP_BasePawn.BP_BasePawn_C|SetObjectType _basepawn (Utilities|Array|MakeArray "ObjectTypeQuery9"))
  (Utilities|IsValid _basepawn
    (:Is%20Valid
      (CallFunction|Setup))))

(event Custom|Setup
  (bind _basepawn (Variables|Default|GetBasePawn))
  (bind _camera (Variables|/Game/FramearqTemplate/Blueprints/Pawn/BP_BasePawn.BP_BasePawn_C|GetCamera _basepawn))
  (bind _returnvalue (Transformation|GetWorldTransform _camera))
  ;[1 1 1] Set photo Frame Location
  (Variables|Default|SetPhotoTransform (Math|Transform|MakeTransform (.location _returnvalue) (.rotation _returnvalue) (Math|Conversions|ToVector(Float) (Variables|/Game/FramearqTemplate/Blueprints/Pawn/BP_BasePawn.BP_BasePawn_C|GetCurrentWorldScale _basepawn))))
  ;[1 1 1] Delete previous BP Photo
  (bind _outactors (Actor|GetAllActorsOfClass "/Game/FramearqTemplate/Blueprints/Commands/Snapshot/BPs/BP_Photo.BP_Photo_C"))
  (Actor|DestroyActor _outactors)
  ;[1 1 1] Create new BP Photo
  (bind _returnvalue_2 (Game|SpawnActorfromClass "/Game/FramearqTemplate/Blueprints/Commands/Snapshot/BPs/BP_Photo.BP_Photo_C" (Variables|Default|GetPhotoTransform) "Undefined" "OverrideRootScale" 0 0))
  (Default|Init _returnvalue_2)
  (Variables|Default|SetCurrentPhotoFrame _returnvalue_2))

(event Custom|Bind_Options
  (bind _optionsbuttons (Variables|Default|GetOptionsButtons))
  (bind _output (Utilities|Array|Get(acopy) _optionsbuttons))
  ;[0.3384 0.6313 1] Setup Option Buttons
  (Variables|/Game/FramearqTemplate/UMG/GameMenu/Option_Button.Option_Button_C|SetWhenExecute _output "NewEnumerator0")
  (EventDispatchers|BindEventtoExecute _output (delegate Custom|Option1))
  (EventDispatchers|BindEventtoEnabled _output (delegate Custom|Enabled))
  (EventDispatchers|BindEventtoDisabled _output (delegate Custom|OnDisable))
  (Game|AssignOnDestroyed (Game|Player|GetPlayerPawn 0) (delegate Custom|OnDestroyed)))

(event Custom|OnDisable
  (bind _returnvalue (Game|Player|GetPlayerPawn 0))
  (bind _currentphotoframe (Variables|Default|GetCurrentPhotoFrame))
  (bind _basepawn (Variables|Default|GetBasePawn))
  (bind _returnvalue_2 (Actor|GetComponentbyClass _returnvalue "/Game/FramearqTemplate/Blueprints/Commands/Transform/BP_TransformComponent.BP_TransformComponent_C"))
  ;[0.3384 0.6313 1] Setup Option Buttons
  (Variables|Default|SetActivated false)
  (Variables|/Game/FramearqTemplate/Blueprints/Pawn/BP_BasePawn.BP_BasePawn_C|SetObjectType _basepawn (Utilities|Array|MakeArray "ObjectTypeQuery1" "ObjectTypeQuery2"))
  (Variables|/Script/Engine.CameraComponent|SetFieldOfView (Variables|/Game/FramearqTemplate/Blueprints/Pawn/BP_BasePawn.BP_BasePawn_C|GetCamera _basepawn) 9e+01)
  (Utilities|IsValid _returnvalue
    (:Is%20Valid
      (Default|SetupTransformComponent _returnvalue_2 false false false false)
      (Variables|/Game/FramearqTemplate/Blueprints/Commands/Transform/BP_TransformComponent.BP_TransformComponent_C|SetIs_L_Updating _returnvalue_2 false)
      (Variables|/Game/FramearqTemplate/Blueprints/Commands/Transform/BP_TransformComponent.BP_TransformComponent_C|SetIs_R_Updating _returnvalue_2 false)
      (Utilities|IsValid _currentphotoframe
        (:Is%20Valid
          (Actor|DestroyActor _currentphotoframe))))))

(event Custom|Option1
  (params (id :type Integer) (Actor :type Actor%20Object%20Reference) (IsRightHand :type Boolean))
  ;[0.3384 0.6313 1] Setup Option Buttons
  (switch Utilities|FlowControl|Switch|SwitchonPV_NavigationMode (Variables|/Game/FramearqTemplate/Blueprints/GameInstance/BP_CollaborativeViewer_GameInstance.BP_CollaborativeViewer_GameInstance_C|GetNavigationMode (.AsBP%20Collaborative%20Viewer%20Game%20Instance (Utilities|Casting|CastToBP_CollaborativeViewer_GameInstance (Game|GetGameInstance))))
    (:NewEnumerator0
      _)
    (:NewEnumerator3
      _)
    (:NewEnumerator1
      _)
    (:NewEnumerator2
      _))
  (Default|DoCapture (Variables|Default|GetCurrentPhotoFrame)))

(event Custom|LeftMousePressed
  (params (Actor :type Actor%20Object%20Reference) (RightHand :type Boolean))
  ;[0 1 0.1488] BeginPlay
  ;;[1 1 1] Binding Button
)

(event Custom|OnDestroyed
  (params (DestroyedActor :type Actor%20Object%20Reference))
  (bind _currentphotoframe (Variables|Default|GetCurrentPhotoFrame))
  ;[0.3384 0.6313 1] Setup Option Buttons
  (Utilities|IsValid _currentphotoframe
    (:Is%20Valid
      (Actor|DestroyActor _currentphotoframe))))

(event EventExecuteAfterSpawnPawn
  ;[0 1 0.1488] BeginPlay
  (if (Utilities|Enum|Equal(Enum) (Game|GetPlatformName) "Windows")
    (Variables|Default|SetIcon "/Game/FramearqTemplate/Blueprints/Commands/Snapshot/IconSnapshot.IconSnapshot")
    (Variables|Default|SetOptionsButtonNames (Utilities|Array|MakeArray "Tomar foto"))
    (Variables|Default|SetName "Instantánea")
    (CallFunction|SetBasePawn)
    (CallFunction|CreateContextualButon false false false)
    (CallFunction|BindOptions)
    (EventDispatchers|BindEventtoMouseLeftPressed (Variables|Default|GetBasePawn) (delegate Custom|LeftMousePressed))))