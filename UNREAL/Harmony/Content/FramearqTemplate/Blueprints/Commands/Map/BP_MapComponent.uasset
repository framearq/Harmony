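; Map command component that adds a "Plano" contextual button to show the floor plan from the player's menu.
; Show and hide call the local pawn, with opening branching between VR (headset detection) and non-VR map views, then restarting the menu.
; When the pawn's TeleportGroupButtonMenu flag is set, both route through authority-switched MTC/ROS events, apparently to sync the map across the group.
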(event Custom|Show%20Plan
  (params (id :type Integer) (Actor :type Actor%20Object%20Reference) (IsRightHand :type Boolean))
  (bind _asbp_base_pawn (Utilities|Casting|CastToBP_BasePawn (Game|Player|GetPlayerPawn 0)))
  (if (Variables|/Game/FramearqTemplate/Blueprints/Pawn/BP_BasePawn.BP_BasePawn_C|GetTeleport_group_Button_menu _asbp_base_pawn)
    (Networking|SwitchHasAuthority
      (:Authority
        (CallFunction|OpenMapMTC))
      (:Remote
        (CallFunction|OpenMapROS)))
    (else
      (if (Math|Boolean|ORBoolean (Class|HeadMountedDisplayFunctionLibrary|IsHeadMountedDisplayEnabled) (and (Utilities|Enum|Equal(Enum) (Game|GetPlatformName) "Android") (Utilities|Name|NotEqual(Name) (Class|HeadMountedDisplayFunctionLibrary|GetHMDDeviceName) "None")) (== (Class|HeadMountedDisplayFunctionLibrary|GetHMDWornState) 1))
        (bind _asbp_vrpawn (Utilities|Casting|CastToBP_VRPawn (Game|Player|GetPlayerPawn 0)))
        (Default|OpenMapPlan _asbp_vrpawn)
        (Default|MenuVisibilityVR _asbp_vrpawn)
        (else
          (bind _asbp_base_pawn_2 (Utilities|Casting|CastToBP_BasePawn (Game|Player|GetPlayerPawn 0)))
          (Default|OpenMapNotVR _asbp_base_pawn_2)
          (Default|HideContextualMenu _asbp_base_pawn_2)))
      ;[1 1 1] restart laser
      (Default|RestartMenu (.AsBP%20Base%20Pawn (Utilities|Casting|CastToBP_BasePawn (Game|Player|GetPlayerPawn 0)))))))

(event Custom|HidePlan_
  (bind _asbp_base_pawn (Utilities|Casting|CastToBP_BasePawn (Game|Player|GetPlayerPawn 0)))
  (if (Variables|/Game/FramearqTemplate/Blueprints/Pawn/BP_BasePawn.BP_BasePawn_C|GetTeleport_group_Button_menu _asbp_base_pawn)
    (Networking|SwitchHasAuthority
      (:Authority
        (CallFunction|CloseMapMTC))
      (:Remote
        (CallFunction|CloseMapROS)))
    (else
      (bind _asbp_base_pawn_2 (Utilities|Casting|CastToBP_BasePawn (Game|Player|GetPlayerPawn 0)))
      (Default|RestartMenu _asbp_base_pawn_2)
      (bind _asbp_vrpawn (Utilities|Casting|CastToBP_VRPawn (Game|Player|GetPlayerPawn 0))
        (:then
          (Default|CloseMapPlan _asbp_vrpawn))
        (:CastFailed
          _))
      (bind _asbp_base_pawn_3 (Utilities|Casting|CastToBP_BasePawn (Game|Player|GetPlayerPawn 0)))
      (Default|CloseMapNotVR _asbp_base_pawn_3))))

(event Custom|Close%20Map%20MTC
  (bind _asbp_base_pawn (Utilities|Casting|CastToBP_BasePawn (Game|Player|GetPlayerPawn 0)))
  (Default|RestartMenu _asbp_base_pawn)
  (bind _asbp_vrpawn (Utilities|Casting|CastToBP_VRPawn (Game|Player|GetPlayerPawn 0))
    (:then
      (Default|CloseMapPlan _asbp_vrpawn))
    (:CastFailed
      _))
  (bind _asbp_base_pawn_2 (Utilities|Casting|CastToBP_BasePawn (Game|Player|GetPlayerPawn 0)))
  (Default|CloseMapNotVR _asbp_base_pawn_2))

(event Custom|Close%20map%20ROS
  (CallFunction|CloseMapMTC))

(event Custom|mostrar%20planta
  (bind _asbp_base_pawn (Utilities|Casting|CastToBP_BasePawn (Game|Player|GetPlayerPawn 0)))
  (if (Variables|/Game/FramearqTemplate/Blueprints/Pawn/BP_BasePawn.BP_BasePawn_C|GetTeleport_group_Button_menu _asbp_base_pawn)
    (Networking|SwitchHasAuthority
      (:Authority
        (CallFunction|OpenMapMTC))
      (:Remote
        (CallFunction|OpenMapROS)))
    (else
      (if (Math|Boolean|ORBoolean (Class|HeadMountedDisplayFunctionLibrary|IsHeadMountedDisplayEnabled) (and (Utilities|Enum|Equal(Enum) (Game|GetPlatformName) "Android") (Utilities|Name|NotEqual(Name) (Class|HeadMountedDisplayFunctionLibrary|GetHMDDeviceName) "None")) (== (Class|HeadMountedDisplayFunctionLibrary|GetHMDWornState) 1))
        (bind _asbp_vrpawn (Utilities|Casting|CastToBP_VRPawn (Game|Player|GetPlayerPawn 0)))
        (Default|OpenMapPlan _asbp_vrpawn)
        (Default|MenuVisibilityVR _asbp_vrpawn)
        (else
          (bind _asbp_base_pawn_2 (Utilities|Casting|CastToBP_BasePawn (Game|Player|GetPlayerPawn 0)))
          (Default|OpenMapNotVR _asbp_base_pawn_2)
          (Default|HideContextualMenu _asbp_base_pawn_2)))
      ;[1 1 1] restart laser
      (Default|RestartMenu (.AsBP%20Base%20Pawn (Utilities|Casting|CastToBP_BasePawn (Game|Player|GetPlayerPawn 0)))))))

(event Custom|Open%20Map%20ROS
  (CallFunction|OpenMapMTC))

(event Custom|Bind_Options
  (bind _optionsbuttons (Variables|Default|GetOptionsButtons))
  (bind _output (Utilities|Array|Get(acopy) _optionsbuttons))
  (Utilities|FlowControl|Sequence
    (:then_0
      (Variables|/Game/FramearqTemplate/UMG/GameMenu/Option_Button.Option_Button_C|SetWhenExecute _output "NewEnumerator1")
      (EventDispatchers|BindEventtoExecute _output (delegate Custom|Show%20Plan)))
    (:then_1
      (EventDispatchers|BindEventtoPressButton (Variables|Default|GetButtonWidget) (delegate Custom|mostrar%20planta)))))

(event Custom|Open%20Map%20MTC
  (if (Math|Boolean|ORBoolean (Class|HeadMountedDisplayFunctionLibrary|IsHeadMountedDisplayEnabled) (and (Utilities|Enum|Equal(Enum) (Game|GetPlatformName) "Android") (Utilities|Name|NotEqual(Name) (Class|HeadMountedDisplayFunctionLibrary|GetHMDDeviceName) "None")) (== (Class|HeadMountedDisplayFunctionLibrary|GetHMDWornState) 1))
    (bind _asbp_vrpawn (Utilities|Casting|CastToBP_VRPawn (Game|Player|GetPlayerPawn 0)))
    (Default|OpenMapPlan _asbp_vrpawn)
    (Default|MenuVisibilityVR _asbp_vrpawn)
    (else
      (bind _asbp_base_pawn (Utilities|Casting|CastToBP_BasePawn (Game|Player|GetPlayerPawn 0)))
      (Default|OpenMapNotVR _asbp_base_pawn)
      (Default|HideContextualMenu _asbp_base_pawn)))
  ;[1 1 1] restart laser
  (Default|RestartMenu (.AsBP%20Base%20Pawn (Utilities|Casting|CastToBP_BasePawn (Game|Player|GetPlayerPawn 0)))))

(event EventBeginPlay)

(event EventExecuteAfterSpawnPawn
  ;[0 1 0.1488] BeginPlayAfterSpawn
  (Variables|Default|SetIcon "/Game/FramearqTemplate/UMG/Textures/map.map")
  (Variables|Default|SetOptionsButtonNamesIcon (Utilities|Array|MakeArray (Utilities|Struct|MakeOption_button_names_icon "Mostrar planta" "/Game/FramearqTemplate/UMG/Textures/arrow_forward_ios.arrow_forward_ios")))
  (Variables|Default|SetName "Plano")
  (CallFunction|SetBasePawn)
  (CallFunction|CreateContextualButon true false false)
  (CallFunction|BindOptions))

(fn OnRepPlan)