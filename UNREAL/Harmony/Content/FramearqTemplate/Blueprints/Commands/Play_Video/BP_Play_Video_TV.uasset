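; Menu command that plays or stops a video on all TV screen actors in the level.
; After pawn spawn it gathers the screens and creates a contextual button with play and stop options.
; Each option runs through ROS and MTC events, apparently server-to-multicast, to open or close the media player.
; These events also swap screen materials, set the pawn's media volume and restart its menu.
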(event Custom|ON%20Stream
  (params (id :type Integer) (Actor :type Actor%20Object%20Reference) (IsRightHand :type Boolean))
  (CallFunction|PlayROS (Variables|Default|GetTV%20Screen)))

(event Custom|OFF%20Stream
  (params (id :type Integer) (Actor :type Actor%20Object%20Reference) (IsRightHand :type Boolean))
  (CallFunction|CloseROS (Variables|Default|GetTV%20Screen)))

(event Custom|Play%20ROS
  (params (TV_Screen :type Array%20of%20TV%20Plane%20Video%20Blueprint%20Object%20References))
  (CallFunction|PlayMTC TV_Screen))

(event Custom|Play%20MTC
  (params (TV_Screen :type Array%20of%20TV%20Plane%20Video%20Blueprint%20Object%20References))
  (Class|MediaPlayer|OpenPlaylistIndex (Variables|Streaming|GetTvMediaPlayer) "/Game/FramearqTemplate/Blueprints/Commands/Play_Video/MediaPlaylist.MediaPlaylist")
  (for _array_element TV_Screen
    (Rendering|Material|SetMaterial (Variables|/Script/Engine.StaticMeshActor|GetStaticMeshComponent _array_element) 0 "/Game/FramearqTemplate/Blueprints/Commands/Play_Video/M_StreamMediaPlayer_Video_Mat.M_StreamMediaPlayer_Video_Mat")
    (bind _asbp_base_pawn (Utilities|Casting|CastToBP_BasePawn (Game|Player|GetPlayerPawn 0)))
    (Audio|Components|Audio|SetVolumeMultiplier (Variables|/Game/FramearqTemplate/Blueprints/Pawn/BP_BasePawn.BP_BasePawn_C|GetMediaSound _asbp_base_pawn) 1.0 :!class /Script/AudioMixer.SynthComponent)
    (bind _asbp_base_pawn_2 (Utilities|Casting|CastToBP_BasePawn (Game|Player|GetPlayerPawn 0)))
    (Default|RestartMenu _asbp_base_pawn_2)))

(event Custom|Close%20ROS
  (params (Tv%20Screen :type Array%20of%20TV%20Plane%20Video%20Blueprint%20Object%20References))
  (CallFunction|CloseMTC Tv%20Screen))

(event Custom|Close%20MTC
  (params (NewParam :type Array%20of%20TV%20Plane%20Video%20Blueprint%20Object%20References))
  (Media|MediaPlayer|Close (Variables|Streaming|GetTvMediaPlayer) :!class /Script/MediaAssets.MediaPlayer)
  (for _array_element NewParam
    (Rendering|Material|SetMaterial (Variables|/Script/Engine.StaticMeshActor|GetStaticMeshComponent _array_element) 0 "/Game/FramearqTemplate/Blueprints/Commands/Play_Video/M_TV_OFF.M_TV_OFF")
    (bind _asbp_base_pawn (Utilities|Casting|CastToBP_BasePawn (Game|Player|GetPlayerPawn 0)))
    (Audio|Components|Audio|SetVolumeMultiplier (Variables|/Game/FramearqTemplate/Blueprints/Pawn/BP_BasePawn.BP_BasePawn_C|GetMediaSound _asbp_base_pawn) 0.0 :!class /Script/AudioMixer.SynthComponent)
    (bind _asbp_base_pawn_2 (Utilities|Casting|CastToBP_BasePawn (Game|Player|GetPlayerPawn 0)))
    (Default|RestartMenu _asbp_base_pawn_2)))

(event Custom|Bind_Options
  (bind _optionsbuttons (Variables|Default|GetOptionsButtons))
  (bind _optionsbuttons_2 (Variables|Default|GetOptionsButtons))
  (bind _output (Utilities|Array|Get(acopy) _optionsbuttons))
  (bind _output_2 (Utilities|Array|Get(acopy) _optionsbuttons_2 1))
  (Utilities|FlowControl|Sequence
    (:then_0
      (Variables|/Game/FramearqTemplate/UMG/GameMenu/Option_Button.Option_Button_C|SetWhenExecute _output "NewEnumerator1")
      (EventDispatchers|BindEventtoExecute _output (delegate Custom|ON%20Stream)))
    (:then_1
      (Variables|/Game/FramearqTemplate/UMG/GameMenu/Option_Button.Option_Button_C|SetWhenExecute _output_2 "NewEnumerator1")
      (EventDispatchers|BindEventtoExecute _output_2 (delegate Custom|OFF%20Stream)))))

(event EventExecuteAfterSpawnPawn
  ;[0 1 0.1488] BeginPlayAfterSpawn
  (bind _outactors (Actor|GetAllActorsOfClass "/Game/FramearqTemplate/Blueprints/Commands/Play_Video/TV_plane_video_Blueprint.TV_plane_video_Blueprint_C"))
  (Variables|Default|SetTV%20Screen _outactors)
  (Variables|Default|SetIcon "/Game/FramearqTemplate/Blueprints/Commands/Play_Video/tv-icon.tv-icon")
  (Variables|Default|SetOptions (Utilities|Array|MakeArray "Reproducir Video TV" "Parar Video TV"))
  (Variables|Default|SetOptionsButtonNames (Variables|Default|GetOptions))
  (Variables|Default|SetName "Video")
  (CallFunction|SetBasePawn)
  (CallFunction|CreateContextualButon false false false)
  (bind _returnvalue (UserInterface|CreateWidget "/Game/FramearqTemplate/Blueprints/Commands/Stream/W_Stream_HUD.W_Stream_HUD_C"))
  (Variables|Streaming|SetWidget%20Stream%20HUD _returnvalue)
  (CallFunction|BindOptions))

(fn ShowLoadindScreen
  (if (Math|Boolean|ORBoolean (Class|HeadMountedDisplayFunctionLibrary|IsHeadMountedDisplayEnabled) (and (Utilities|Enum|Equal(Enum) (Game|GetPlatformName) "Android") (Utilities|Name|NotEqual(Name) (Class|HeadMountedDisplayFunctionLibrary|GetHMDDeviceName) "None")) (== (Class|HeadMountedDisplayFunctionLibrary|GetHMDWornState) 1))
    (Class|XRLoadingScreenFunctionLibrary|AddLoadingScreenSplash "/Game/FramearqTemplate/UMG/Textures/pantalla-carga-VR.pantalla-carga-VR" "1.000000,0.000000,1.500000" "0, 0, 0" "(X=1.500000,Y=1.500000)" "0, 0, 0" true)
    (Class|XRLoadingScreenFunctionLibrary|ShowLoadingScreen)
    (else
      (bind _returnvalue (UserInterface|CreateWidget "/Game/FramearqTemplate/UMG/GameMenu/pantalla_carga.pantalla_carga_C"))
      (UserInterface|Viewport|AddtoViewport _returnvalue 0))))

(fn OnRepIsDay?)

(fn CheckVR/AndroidorPC
  (return (Math|Boolean|ORBoolean (Class|HeadMountedDisplayFunctionLibrary|IsHeadMountedDisplayEnabled) (and (Utilities|Enum|Equal(Enum) (Game|GetPlatformName) "Android") (Utilities|Name|NotEqual(Name) (Class|HeadMountedDisplayFunctionLibrary|GetHMDDeviceName) "None")) (== (Class|HeadMountedDisplayFunctionLibrary|GetHMDWornState) 1))))