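; BP_EditableObject is an actor whose mesh carries a default color and material, apparently for the template's material-editing commands.
; The construction script applies the configured static mesh, creates a dynamic instance of the default material on slot 0 and sets its Color parameter.
; SetInitialState stores a self reference with the default color, material, brush and names in InitialStateVariables.
; The event graph has no other active logic.
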(event Custom|Set%20Initial%20State
  (Variables|Default|SetInitialStateVariables (Utilities|Struct|MakeInitialState self (Variables|OpcionesDefault|GetDefaultColor) (Variables|OpcionesDefault|GetDefault%20color%20name) (Variables|OpcionesDefault|GetDefaultColorMaterial) (Variables|OpcionesDefault|GetDefaultMaterialBrush) (Variables|OpcionesDefault|GetDefault%20Material%20Name))))

(event EventBeginPlay)

(event Collision|EventActorBeginOverlap
  (params (OtherActor :type Actor%20Object%20Reference)))

(event EventTick
  (params (DeltaSeconds :type Float%20%28single-precision%29)))

(fn ConstructionScript
  (bind _mesh_object (Variables|Default|GetMesh_object))
  (Components|StaticMesh|SetStaticMesh _mesh_object (Variables|Default|GetMesh%20object%20to%20edit))
  (bind _returnvalue (Rendering|Material|CreateDynamicMaterialInstance _mesh_object 0 (Variables|OpcionesDefault|GetDefaultColorMaterial) "None" :!class /Script/Engine.PrimitiveComponent))
  (Rendering|Material|SetVectorParameterValue _returnvalue "Color" (Variables|OpcionesDefault|GetDefaultColor) :!class /Script/Engine.MaterialInstanceDynamic))