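; XrayManager keeps the registry of actors used by the X-ray command, along with a snapshot of their materials.
; AddXrayActor skips invalid or already registered actors, then gathers materials from all the actor's StaticMeshComponents into one entry in MaterialsArrays, stored parallel to XrayActors.
; AddArrayXrayActor registers actors in batches, and ClearXrayActors empties both arrays.
; No material swapping or restoring happens in this Blueprint.
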(event Custom|ClearXrayActors
  (Utilities|Array|Clear (Variables|Default|GetXrayActors))
  (Utilities|Array|Clear (Variables|Default|GetMaterialsArrays)))

(event Custom|AddXrayActor
  (params (XrayActor :type Actor%20Object%20Reference%20%28by%20ref%29))
  (Utilities|IsValid XrayActor
    (:Is%20Valid
      (if (not (Utilities|Array|ContainsItem (Variables|Default|GetXrayActors) XrayActor))
        (for _array_element (Actor|GetComponentsByClass XrayActor "/Script/Engine.StaticMeshComponent")
          (Utilities|Array|AppendArray (Variables|Default|GetCurrentActorMaterials) (Rendering|Material|GetMaterials _array_element)))
        (Utilities|Array|Add (Variables|Default|GetXrayActors) XrayActor)
        (Utilities|Array|Add (Variables|Default|GetMaterialsArrays) (Utilities|Struct|MakeXrayMaterialsArrays (Variables|Default|GetCurrentActorMaterials)))
        (Utilities|Array|Clear (Variables|Default|GetCurrentActorMaterials))))))

(event Custom|AddArrayXrayActor
  (params (XrayActorsArray :type Array%20of%20Actor%20Object%20References))
  (for _array_element XrayActorsArray
    (CallFunction|AddXrayActor _array_element)))

(event EventBeginPlay)

(event Collision|EventActorBeginOverlap
  (params (OtherActor :type Actor%20Object%20Reference)))

(event EventTick
  (params (DeltaSeconds :type Float%20%28single-precision%29)))

(fn ConstructionScript)