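; Command that adds a "Modo sentado" toggle button to the player controller's contextual widget bar to switch between standing and sitting modes.
; On release it flips PlayerModes in the game instance, updates the button state and passes the change to the VR pawn or login-menu pawn.
; The choice persists in the SaveOptions save slot, which is read back on spawn to set the game instance and button state.
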(event Custom|Set%20button%20status
  (bind _button_settings (Variables|Default|GetButton%20Settings))
  (bind _button_settings_2 (Variables|Default|GetButton%20Settings))
  ;[1 1 1] Load
  (bind _returnvalue (SaveGame|DoesSaveGameExist (Variables|Default|GetSave_options)))
  (if _returnvalue
    (bind _returnvalue_2 (SaveGame|LoadGamefromSlot (Variables|Default|GetSave_options)))
    (bind _asbp_save_player_options (Utilities|Casting|CastToBP_Save_player_options _returnvalue_2))
    (bind _asbp_collaborative_viewer_game_instance (Utilities|Casting|CastToBP_CollaborativeViewer_GameInstance (Game|GetGameInstance)))
    (Variables|/Game/FramearqTemplate/Blueprints/GameInstance/BP_CollaborativeViewer_GameInstance.BP_CollaborativeViewer_GameInstance_C|SetPlayer_modes _asbp_collaborative_viewer_game_instance (Variables|/Game/FramearqTemplate/Blueprints/SaveGame/BP_Save_player_options.BP_Save_player_options_C|GetPlayer_mode _asbp_save_player_options)))
  (bind _asbp_collaborative_viewer_game_instance_2 (Utilities|Casting|CastToBP_CollaborativeViewer_GameInstance (Game|GetGameInstance)))
  (switch Utilities|FlowControl|Switch|SwitchonE_player_modes (Variables|/Game/FramearqTemplate/Blueprints/GameInstance/BP_CollaborativeViewer_GameInstance.BP_CollaborativeViewer_GameInstance_C|GetPlayer_modes _asbp_collaborative_viewer_game_instance_2)
    (:NewEnumerator0
      (Development|PrintString "De pie")
      (Variables|/Game/FramearqTemplate/UMG/GameMenu/Settings_button.Settings_button_C|SetButton_status _button_settings (Utilities|Array|Get(acopy) (Variables|Default|GetButton%20States)))
      (Variables|Default|Setplayer_mode_widget "NewEnumerator0")
      (Variables|/Game/FramearqTemplate/UMG/GameMenu/Settings_button.Settings_button_C|SetEnable%20state _button_settings_2 false))
    (:NewEnumerator1
      (Development|PrintString "Sentado")
      (Variables|/Game/FramearqTemplate/UMG/GameMenu/Settings_button.Settings_button_C|SetButton_status _button_settings (Utilities|Array|Get(acopy) (Variables|Default|GetButton%20States) 1))
      (Variables|Default|Setplayer_mode_widget "NewEnumerator1")
      (Variables|/Game/FramearqTemplate/UMG/GameMenu/Settings_button.Settings_button_C|SetEnable%20state _button_settings_2 true))))

(event Custom|Released%20Button
  (bind _returnvalue (Game|Player|GetPlayerPawn 0))
  (bind _returnvalue_2 (Game|Player|GetPlayerPawn 0))
  (bind _button_settings (Variables|Default|GetButton%20Settings))
  (bind _button_settings_2 (Variables|Default|GetButton%20Settings))
  (bind _asbp_collaborative_viewer_game_instance (Utilities|Casting|CastToBP_CollaborativeViewer_GameInstance (Game|GetGameInstance)))
  (switch Utilities|FlowControl|Switch|SwitchonE_player_modes (Variables|/Game/FramearqTemplate/Blueprints/GameInstance/BP_CollaborativeViewer_GameInstance.BP_CollaborativeViewer_GameInstance_C|GetPlayer_modes _asbp_collaborative_viewer_game_instance)
    (:NewEnumerator0
      (Development|PrintString "Sentado")
      (Variables|/Game/FramearqTemplate/UMG/GameMenu/Settings_button.Settings_button_C|SetButton_status _button_settings_2 (Utilities|Array|Get(acopy) (Variables|Default|GetButton%20States) 1))
      (Variables|/Game/FramearqTemplate/UMG/GameMenu/Settings_button.Settings_button_C|SetEnable%20state _button_settings true)
      (bind _asbp_collaborative_viewer_game_instance_2 (Utilities|Casting|CastToBP_CollaborativeViewer_GameInstance (Game|GetGameInstance)))
      (Variables|/Game/FramearqTemplate/Blueprints/GameInstance/BP_CollaborativeViewer_GameInstance.BP_CollaborativeViewer_GameInstance_C|SetPlayer_modes _asbp_collaborative_viewer_game_instance_2 "NewEnumerator1")
      (Variables|Default|Setplayer_mode_widget "NewEnumerator1")
      (Utilities|FlowControl|Sequence
        (:then_0
          (bind _asbp_vrpawn (Utilities|Casting|CastToBP_VRPawn _returnvalue))
          (Default|SetPlayerModes _asbp_vrpawn true)
          (Variables|/Game/FramearqTemplate/Blueprints/Pawn/VR/BP_VRPawn.BP_VRPawn_C|SetcontextualWidgetOpen _asbp_vrpawn false))
        (:then_1
          (bind _asbp_login_menu_pawn_final (Utilities|Casting|CastToBP_LoginMenu_PawnFinal _returnvalue))
          (Default|SetPlayerMode _asbp_login_menu_pawn_final true))
        (:then_2
          ;[1 1 1] save mode
          (bind _returnvalue_3 (SaveGame|DoesSaveGameExist (Variables|Default|GetSave_options) :!label _label))
          (if _returnvalue_3
            (bind _returnvalue_4 (SaveGame|LoadGamefromSlot (Variables|Default|GetSave_options)))
            (Variables|Default|SetSave_game_mode _returnvalue_4)
            (else
              (bind _returnvalue_5 (SaveGame|CreateSaveGameObject "/Game/FramearqTemplate/Blueprints/SaveGame/BP_Save_player_options.BP_Save_player_options_C"))
              (Variables|Default|SetSave_game_mode _returnvalue_5)))
          (bind _asbp_save_player_options (Utilities|Casting|CastToBP_Save_player_options (Variables|Default|GetSave_game_mode)))
          (Variables|/Game/FramearqTemplate/Blueprints/SaveGame/BP_Save_player_options.BP_Save_player_options_C|SetPlayer_mode _asbp_save_player_options (Variables|Default|Getplayer_mode_widget))
          (SaveGame|SaveGametoSlot (Variables|Default|GetSave_game_mode) (Variables|Default|GetSave_options)))))
    (:NewEnumerator1
      (Development|PrintString "De pie")
      (Variables|/Game/FramearqTemplate/UMG/GameMenu/Settings_button.Settings_button_C|SetButton_status _button_settings_2 (Utilities|Array|Get(acopy) (Variables|Default|GetButton%20States)))
      (Variables|/Game/FramearqTemplate/UMG/GameMenu/Settings_button.Settings_button_C|SetEnable%20state _button_settings false)
      (bind _asbp_collaborative_viewer_game_instance_3 (Utilities|Casting|CastToBP_CollaborativeViewer_GameInstance (Game|GetGameInstance)))
      (Variables|/Game/FramearqTemplate/Blueprints/GameInstance/BP_CollaborativeViewer_GameInstance.BP_CollaborativeViewer_GameInstance_C|SetPlayer_modes _asbp_collaborative_viewer_game_instance_3 "NewEnumerator0")
      (Variables|Default|Setplayer_mode_widget "NewEnumerator0")
      (Utilities|FlowControl|Sequence
        (:then_0
          (bind _asbp_vrpawn_2 (Utilities|Casting|CastToBP_VRPawn _returnvalue_2))
          (Default|SetPlayerModes _asbp_vrpawn_2 false)
          (Variables|/Game/FramearqTemplate/Blueprints/Pawn/VR/BP_VRPawn.BP_VRPawn_C|SetcontextualWidgetOpen _asbp_vrpawn_2 false))
        (:then_1
          (bind _asbp_login_menu_pawn_final_2 (Utilities|Casting|CastToBP_LoginMenu_PawnFinal _returnvalue_2))
          (Default|SetPlayerMode _asbp_login_menu_pawn_final_2 false))
        (:then_2
          (goto _label))))))

(event Custom|Bind%20Events
  (EventDispatchers|BindEventtoOnReleasedButton (Variables|Default|GetButton%20Settings) (delegate Custom|Released%20Button)))

(event EventExecuteAfterSpawnPawn
  (bind _returnvalue (Game|GetPlayerController 0))
  ;[0 1 0.1488] BeginPlayAfterSpawn (Insert button texts and icon)
  (Variables|Default|SetButton%20States (Utilities|Array|MakeArray "Desactivado" "Activado"))
  (Variables|Default|SetButton%20text "Modo sentado")
  (Variables|Default|SetButton%20icon "/Game/FramearqTemplate/UMG/Textures/T_icon_sitting.T_icon_sitting")
  (bind _asbp_collab_v_player_controller (Utilities|Casting|CastToBP_Collab_V_PlayerController _returnvalue))
  (bind _returnvalue_2 (UserInterface|CreateWidget "/Game/FramearqTemplate/UMG/GameMenu/Settings_button.Settings_button_C" _returnvalue (Variables|Default|GetButton%20icon) (Variables|Default|GetButton%20text)))
  (bind _output_get (Variables|Default|SetButton%20Settings _returnvalue_2))
  (Class|HorizontalBox|AddChildtoHorizontalBox (Variables|/Game/FramearqTemplate/UMG/GameMenu/Contextual_Widget.Contextual_Widget_C|GetSecundary_Bar_Box (Variables|/Game/FramearqTemplate/Blueprints/PlayerController/BP_Collab_V_PlayerController.BP_Collab_V_PlayerController_C|GetContextualWidget _asbp_collab_v_player_controller)) _output_get)
  (CallFunction|BindEvents)
  (CallFunction|SetButtonStatus))