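; Day/night menu command that offers "Día" and "Noche" options through a contextual button created after the pawn spawns.
; Each option restarts the pawn menu, then calls a ROS event that forwards to its MTC counterpart.
; Both MTC events are empty here: the camera fade, streaming-level swap and sky dome intensity chains are left unconnected.
; A separate function shows a VR splash or widget loading screen.
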(event Custom|Go%20to%20Day
  (params (id :type Integer) (Actor :type Actor%20Object%20Reference) (IsRightHand :type Boolean))
  (Default|RestartMenu (.AsBP%20Base%20Pawn (Utilities|Casting|CastToBP_BasePawn (Game|Player|GetPlayerPawn 0))))
  (CallFunction|ToDayROS))

(event Custom|Close%20Night
  (params (id :type Integer) (Actor :type Actor%20Object%20Reference) (IsRightHand :type Boolean))
  (Default|RestartMenu (.AsBP%20Base%20Pawn (Utilities|Casting|CastToBP_BasePawn (Game|Player|GetPlayerPawn 0))))
  (CallFunction|ToNightROS))

(event Custom|to%20Day%20MTC
  ;[1 1 1] Fade Out
)

(event Custom|to%20Day%20ROS
  (CallFunction|ToDayMTC))

(event Custom|to%20Night%20MTC
  ;[1 1 1] Fade Out
)

(event Custom|to%20Night%20ROS
  (CallFunction|ToNightMTC))

(event Custom|Bind_Options
  (bind _optionsbuttons (Variables|Default|GetOptionsButtons))
  (bind _optionsbuttons_2 (Variables|Default|GetOptionsButtons))
  (bind _output (Utilities|Array|Get(acopy) _optionsbuttons_2 1))
  (bind _output_2 (Utilities|Array|Get(acopy) _optionsbuttons))
  (Utilities|FlowControl|Sequence
    (:then_0
      (Variables|/Game/FramearqTemplate/UMG/GameMenu/Option_Button.Option_Button_C|SetWhenExecute _output_2 "NewEnumerator1")
      (EventDispatchers|BindEventtoExecute _output_2 (delegate Custom|Go%20to%20Day)))
    (:then_1
      (Variables|/Game/FramearqTemplate/UMG/GameMenu/Option_Button.Option_Button_C|SetWhenExecute _output "NewEnumerator1")
      (EventDispatchers|BindEventtoExecute _output (delegate Custom|Close%20Night)))))

(event EventExecuteAfterSpawnPawn
  ;[0 1 0.1488] BeginPlayAfterSpawn
  (Variables|Default|SetIcon "/Game/FramearqTemplate/Blueprints/Commands/Day_Hours/day-night-icon.day-night-icon")
  (Variables|Default|SetOptionsButtonNamesIcon (Utilities|Array|MakeArray (Utilities|Struct|MakeOption_button_names_icon "Día" "/Game/FramearqTemplate/UMG/Textures/arrow_forward_ios.arrow_forward_ios") (Utilities|Struct|MakeOption_button_names_icon "Noche" "/Game/FramearqTemplate/UMG/Textures/arrow_forward_ios.arrow_forward_ios")))
  (Variables|Default|SetName "Dia / Noche")
  (CallFunction|SetBasePawn)
  (CallFunction|CreateContextualButon false false false)
  (CallFunction|BindOptions))

(fn ShowLoadindScreen
  (if (Math|Boolean|ORBoolean (Class|HeadMountedDisplayFunctionLibrary|IsHeadMountedDisplayEnabled) (and (Utilities|Enum|Equal(Enum) (Game|GetPlatformName) "Android") (Utilities|Name|NotEqual(Name) (Class|HeadMountedDisplayFunctionLibrary|GetHMDDeviceName) "None")) (== (Class|HeadMountedDisplayFunctionLibrary|GetHMDWornState) 1))
    (Class|XRLoadingScreenFunctionLibrary|AddLoadingScreenSplash "/Game/FramearqTemplate/UMG/Textures/pantalla-carga-VR.pantalla-carga-VR" "1.000000,0.000000,1.500000" "0, 0, 0" "(X=1.500000,Y=1.500000)" "0, 0, 0" true)
    (Class|XRLoadingScreenFunctionLibrary|ShowLoadingScreen)
    (else
      (bind _returnvalue (UserInterface|CreateWidget "/Game/FramearqTemplate/UMG/GameMenu/pantalla_carga.pantalla_carga_C"))
      (UserInterface|Viewport|AddtoViewport _returnvalue 0))))

(fn OnRepIsDay?)