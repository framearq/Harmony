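; Command that adds an inverted-control ("Control invertido") toggle to the settings secondary bar on Android devices without an HMD.
; After pawn spawn it creates a Settings_button and restores its state from the saved options via the GameInstance's ControlNormal flag.
; Each release flips that flag, updates the Desktop WalkMode pawn's control type and saves the choice.
; An older UI_touch_mode button path remains but never runs.
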(event Custom|Set%20button%20status
  (bind _button_settings (Variables|Default|GetButton%20Settings))
  (bind _button_settings_2 (Variables|Default|GetButton%20Settings))
  ;[1 1 1] Load
  (bind _returnvalue (SaveGame|DoesSaveGameExist (Variables|Default|GetSave_options)))
  (if _returnvalue
    (bind _returnvalue_2 (SaveGame|LoadGamefromSlot (Variables|Default|GetSave_options)))
    (bind _asbp_save_player_options (Utilities|Casting|CastToBP_Save_player_options _returnvalue_2))
    (bind _asbp_collaborative_viewer_game_instance (Utilities|Casting|CastToBP_CollaborativeViewer_GameInstance (Game|GetGameInstance)))
    (Variables|/Game/FramearqTemplate/Blueprints/GameInstance/BP_CollaborativeViewer_GameInstance.BP_CollaborativeViewer_GameInstance_C|SetControl_normal _asbp_collaborative_viewer_game_instance (Variables|/Game/FramearqTemplate/Blueprints/SaveGame/BP_Save_player_options.BP_Save_player_options_C|Getcontrol_normal _asbp_save_player_options)))
  (bind _asbp_collaborative_viewer_game_instance_2 (Utilities|Casting|CastToBP_CollaborativeViewer_GameInstance (Game|GetGameInstance)))
  (if (Variables|/Game/FramearqTemplate/Blueprints/GameInstance/BP_CollaborativeViewer_GameInstance.BP_CollaborativeViewer_GameInstance_C|GetControl_normal _asbp_collaborative_viewer_game_instance_2)
    (Development|PrintString "Normal")
    (Variables|/Game/FramearqTemplate/UMG/GameMenu/Settings_button.Settings_button_C|SetButton_status _button_settings_2 (Utilities|Array|Get(acopy) (Variables|Default|GetButton%20States)))
    (Variables|Default|Setcontrol_normal_widget true)
    (Variables|/Game/FramearqTemplate/UMG/GameMenu/Settings_button.Settings_button_C|SetEnable%20state _button_settings false)
    (else
      (Development|PrintString "Invertido")
      (Variables|/Game/FramearqTemplate/UMG/GameMenu/Settings_button.Settings_button_C|SetButton_status _button_settings_2 (Utilities|Array|Get(acopy) (Variables|Default|GetButton%20States) 1))
      (Variables|Default|Setcontrol_normal_widget false)
      (Variables|/Game/FramearqTemplate/UMG/GameMenu/Settings_button.Settings_button_C|SetEnable%20state _button_settings true))))

(event Custom|Released%20Button
  (bind _button_settings (Variables|Default|GetButton%20Settings))
  (bind _button_settings_2 (Variables|Default|GetButton%20Settings))
  (bind _asbp_collaborative_viewer_game_instance (Utilities|Casting|CastToBP_CollaborativeViewer_GameInstance (Game|GetGameInstance)))
  (if (Variables|/Game/FramearqTemplate/Blueprints/GameInstance/BP_CollaborativeViewer_GameInstance.BP_CollaborativeViewer_GameInstance_C|GetControl_normal _asbp_collaborative_viewer_game_instance)
    (Development|PrintString "Invertido")
    (Variables|/Game/FramearqTemplate/UMG/GameMenu/Settings_button.Settings_button_C|SetButton_status _button_settings_2 (Utilities|Array|Get(acopy) (Variables|Default|GetButton%20States) 1))
    (Variables|/Game/FramearqTemplate/UMG/GameMenu/Settings_button.Settings_button_C|SetEnable%20state _button_settings true)
    (bind _asbp_collaborative_viewer_game_instance_2 (Utilities|Casting|CastToBP_CollaborativeViewer_GameInstance (Game|GetGameInstance)))
    (Variables|/Game/FramearqTemplate/Blueprints/GameInstance/BP_CollaborativeViewer_GameInstance.BP_CollaborativeViewer_GameInstance_C|SetControl_normal _asbp_collaborative_viewer_game_instance_2 false)
    (Variables|Default|Setcontrol_normal_widget false)
    (bind _asbp_desktop_walk_mode_pawn (Utilities|Casting|CastToBP_Desktop_WalkMode_Pawn (Game|Player|GetPlayerPawn 0))
      (:then
        (Default|ControlType _asbp_desktop_walk_mode_pawn false))
      (:CastFailed
        _))
    (else
      (Development|PrintString "Normal")
      (Variables|/Game/FramearqTemplate/UMG/GameMenu/Settings_button.Settings_button_C|SetButton_status _button_settings_2 (Utilities|Array|Get(acopy) (Variables|Default|GetButton%20States)))
      (Variables|/Game/FramearqTemplate/UMG/GameMenu/Settings_button.Settings_button_C|SetEnable%20state _button_settings false)
      (bind _asbp_collaborative_viewer_game_instance_3 (Utilities|Casting|CastToBP_CollaborativeViewer_GameInstance (Game|GetGameInstance)))
      (Variables|/Game/FramearqTemplate/Blueprints/GameInstance/BP_CollaborativeViewer_GameInstance.BP_CollaborativeViewer_GameInstance_C|SetControl_normal _asbp_collaborative_viewer_game_instance_3 true)
      (Variables|Default|Setcontrol_normal_widget true)
      (bind _asbp_desktop_walk_mode_pawn_2 (Utilities|Casting|CastToBP_Desktop_WalkMode_Pawn (Game|Player|GetPlayerPawn 0))
        (:then
          (Default|ControlType _asbp_desktop_walk_mode_pawn_2 true))
        (:CastFailed
          _))))
  (Audio|PlaySound2D "/Game/FramearqTemplate/Sounds/Button_Click.Button_Click" 1.0 1.0 0.0 0 0)
  ;[1 1 1] save mode
  (bind _returnvalue (SaveGame|DoesSaveGameExist (Variables|Default|GetSave_options)))
  (if _returnvalue
    (bind _returnvalue_2 (SaveGame|LoadGamefromSlot (Variables|Default|GetSave_options)))
    (Variables|Default|SetSave_game_mode _returnvalue_2)
    (else
      (bind _returnvalue_3 (SaveGame|CreateSaveGameObject "/Game/FramearqTemplate/Blueprints/SaveGame/BP_Save_player_options.BP_Save_player_options_C"))
      (Variables|Default|SetSave_game_mode _returnvalue_3)))
  (bind _asbp_save_player_options (Utilities|Casting|CastToBP_Save_player_options (Variables|Default|GetSave_game_mode)))
  (Variables|/Game/FramearqTemplate/Blueprints/SaveGame/BP_Save_player_options.BP_Save_player_options_C|Setcontrol_normal _asbp_save_player_options (Variables|Default|Getcontrol_normal_widget))
  (SaveGame|SaveGametoSlot (Variables|Default|GetSave_game_mode) (Variables|Default|GetSave_options)))

(event Custom|Bind%20Events
  (EventDispatchers|BindEventtoOnReleasedButton (Variables|Default|GetButton%20Settings) (delegate Custom|Released%20Button)))

(event EventExecuteAfterSpawnPawn
  (bind _returnvalue (Game|GetPlayerController 0))
  ;[0 1 0.1488] BeginPlayAfterSpawn (Insert button texts and icon)
  (if (and (Utilities|Enum|Equal(Enum) (Game|GetPlatformName) "Android") (not (Utilities|Name|NotEqual(Name) (Class|HeadMountedDisplayFunctionLibrary|GetHMDDeviceName) "None")))
    (Variables|Default|SetButton%20States (Utilities|Array|MakeArray "Desactivado" "Activado"))
    (Variables|Default|SetButton%20text "Control invertido")
    (Variables|Default|SetButton%20icon "/Game/FramearqTemplate/UMG/Textures/control-invertido-icon.control-invertido-icon")
    (bind _asbp_collab_v_player_controller (Utilities|Casting|CastToBP_Collab_V_PlayerController _returnvalue))
    (bind _returnvalue_2 (UserInterface|CreateWidget "/Game/FramearqTemplate/UMG/GameMenu/Settings_button.Settings_button_C" _returnvalue (Variables|Default|GetButton%20icon) (Variables|Default|GetButton%20text)))
    (bind _output_get (Variables|Default|SetButton%20Settings _returnvalue_2))
    (Class|HorizontalBox|AddChildtoHorizontalBox (Variables|/Game/FramearqTemplate/UMG/GameMenu/Contextual_Widget.Contextual_Widget_C|GetSecundary_Bar_Box (Variables|/Game/FramearqTemplate/Blueprints/PlayerController/BP_Collab_V_PlayerController.BP_Collab_V_PlayerController_C|GetContextualWidget _asbp_collab_v_player_controller)) _output_get)
    (CallFunction|BindEvents)
    (CallFunction|SetButtonStatus)))