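; VR settings command that adds a "Mostrar controles" button to the player controller's contextual bar, toggling between controller info and hands.
; On spawn it syncs the GameInstance's ShowInfoControllers flag from the options save, if present, and sets the button state.
; Each release flips the flag, shows or hides the VRPawn tutorial or switches the login-menu pawn between hands and Oculus controller, then saves the option.
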(event Custom|Create%20Bind%20Events
  (EventDispatchers|BindEventtoOnReleasedButton (Variables|Default|GetButton%20Settings) (delegate Custom|Released%20Button)))

(event Custom|Released%20Button
  (bind _button_settings (Variables|Default|GetButton%20Settings))
  (bind _button_settings_2 (Variables|Default|GetButton%20Settings))
  (bind _asbp_collaborative_viewer_game_instance (Utilities|Casting|CastToBP_CollaborativeViewer_GameInstance (Game|GetGameInstance)))
  (if (Variables|/Game/FramearqTemplate/Blueprints/GameInstance/BP_CollaborativeViewer_GameInstance.BP_CollaborativeViewer_GameInstance_C|Getshow_info_controllers _asbp_collaborative_viewer_game_instance)
    (Development|PrintString "Mostrar manos")
    (Variables|/Game/FramearqTemplate/UMG/GameMenu/Settings_button.Settings_button_C|SetButton_status _button_settings_2 (Utilities|Array|Get(acopy) (Variables|Default|GetButton%20States)))
    (Variables|/Game/FramearqTemplate/UMG/GameMenu/Settings_button.Settings_button_C|SetEnable%20state _button_settings false)
    (bind _asbp_collaborative_viewer_game_instance_2 (Utilities|Casting|CastToBP_CollaborativeViewer_GameInstance (Game|GetGameInstance)))
    (Variables|/Game/FramearqTemplate/Blueprints/GameInstance/BP_CollaborativeViewer_GameInstance.BP_CollaborativeViewer_GameInstance_C|Setshow_info_controllers _asbp_collaborative_viewer_game_instance_2 false)
    (Variables|Default|Setshow_info_controllers_widget false)
    (Utilities|FlowControl|Sequence
      (:then_0
        (bind _asbp_vrpawn (Utilities|Casting|CastToBP_VRPawn (Game|Player|GetPlayerPawn 0)))
        (Default|HideTutorial _asbp_vrpawn))
      (:then_1
        (bind _asbp_login_menu_pawn_final (Utilities|Casting|CastToBP_LoginMenu_PawnFinal (Game|Player|GetPlayerPawn 0)))
        (Default|ShowHands _asbp_login_menu_pawn_final))
      (:then_2
        ;[1 1 1] save mode
        (bind _returnvalue (SaveGame|DoesSaveGameExist (Variables|Default|GetSave_options) :!label _label))
        (if _returnvalue
          (bind _returnvalue_2 (SaveGame|LoadGamefromSlot (Variables|Default|GetSave_options)))
          (Variables|Default|SetSave_game_mode _returnvalue_2)
          (else
            (bind _returnvalue_3 (SaveGame|CreateSaveGameObject "/Game/FramearqTemplate/Blueprints/SaveGame/BP_Save_player_options.BP_Save_player_options_C"))
            (Variables|Default|SetSave_game_mode _returnvalue_3)))
        (bind _asbp_save_player_options (Utilities|Casting|CastToBP_Save_player_options (Variables|Default|GetSave_game_mode)))
        (Variables|/Game/FramearqTemplate/Blueprints/SaveGame/BP_Save_player_options.BP_Save_player_options_C|Setshow_info_controllers _asbp_save_player_options (Variables|Default|Getshow_info_controllers_widget))
        (SaveGame|SaveGametoSlot (Variables|Default|GetSave_game_mode) (Variables|Default|GetSave_options))))
    (else
      (Development|PrintString "Mostrar controles")
      (Variables|/Game/FramearqTemplate/UMG/GameMenu/Settings_button.Settings_button_C|SetButton_status _button_settings_2 (Utilities|Array|Get(acopy) (Variables|Default|GetButton%20States) 1))
      (Variables|/Game/FramearqTemplate/UMG/GameMenu/Settings_button.Settings_button_C|SetEnable%20state _button_settings true)
      (bind _asbp_collaborative_viewer_game_instance_3 (Utilities|Casting|CastToBP_CollaborativeViewer_GameInstance (Game|GetGameInstance)))
      (Variables|/Game/FramearqTemplate/Blueprints/GameInstance/BP_CollaborativeViewer_GameInstance.BP_CollaborativeViewer_GameInstance_C|Setshow_info_controllers _asbp_collaborative_viewer_game_instance_3 true)
      (Variables|Default|Setshow_info_controllers_widget true)
      (Utilities|FlowControl|Sequence
        (:then_0
          (bind _asbp_vrpawn_2 (Utilities|Casting|CastToBP_VRPawn (Game|Player|GetPlayerPawn 0)))
          (Default|ShowTutorial _asbp_vrpawn_2))
        (:then_1
          (bind _asbp_login_menu_pawn_final_2 (Utilities|Casting|CastToBP_LoginMenu_PawnFinal (Game|Player|GetPlayerPawn 0)))
          (Default|ShowOculusController _asbp_login_menu_pawn_final_2))
        (:then_2
          (goto _label))))))

(event Custom|Set%20button%20status
  (bind _button_settings (Variables|Default|GetButton%20Settings))
  (bind _button_settings_2 (Variables|Default|GetButton%20Settings))
  ;[1 1 1] Load
  (bind _returnvalue (SaveGame|DoesSaveGameExist (Variables|Default|GetSave_options)))
  (if _returnvalue
    (bind _returnvalue_2 (SaveGame|LoadGamefromSlot (Variables|Default|GetSave_options)))
    (bind _asbp_save_player_options (Utilities|Casting|CastToBP_Save_player_options _returnvalue_2))
    (bind _asbp_collaborative_viewer_game_instance (Utilities|Casting|CastToBP_CollaborativeViewer_GameInstance (Game|GetGameInstance)))
    (Variables|/Game/FramearqTemplate/Blueprints/GameInstance/BP_CollaborativeViewer_GameInstance.BP_CollaborativeViewer_GameInstance_C|Setshow_info_controllers _asbp_collaborative_viewer_game_instance (Variables|/Game/FramearqTemplate/Blueprints/SaveGame/BP_Save_player_options.BP_Save_player_options_C|Getshow_info_controllers _asbp_save_player_options)))
  (bind _asbp_collaborative_viewer_game_instance_2 (Utilities|Casting|CastToBP_CollaborativeViewer_GameInstance (Game|GetGameInstance)))
  (if (Variables|/Game/FramearqTemplate/Blueprints/GameInstance/BP_CollaborativeViewer_GameInstance.BP_CollaborativeViewer_GameInstance_C|Getshow_info_controllers _asbp_collaborative_viewer_game_instance_2)
    (Development|PrintString "Mostrar controles")
    (Variables|/Game/FramearqTemplate/UMG/GameMenu/Settings_button.Settings_button_C|SetButton_status _button_settings_2 (Utilities|Array|Get(acopy) (Variables|Default|GetButton%20States) 1))
    (Variables|Default|Setshow_info_controllers_widget true)
    (Variables|/Game/FramearqTemplate/UMG/GameMenu/Settings_button.Settings_button_C|SetEnable%20state _button_settings true)
    (else
      (Development|PrintString "Mostrar manos")
      (Variables|/Game/FramearqTemplate/UMG/GameMenu/Settings_button.Settings_button_C|SetButton_status _button_settings_2 (Utilities|Array|Get(acopy) (Variables|Default|GetButton%20States)))
      (Variables|Default|Setshow_info_controllers_widget false)
      (Variables|/Game/FramearqTemplate/UMG/GameMenu/Settings_button.Settings_button_C|SetEnable%20state _button_settings false))))

(event EventExecuteAfterSpawnPawn
  (bind _returnvalue (Game|GetPlayerController 0))
  ;[0 1 0.1488] BeginPlayAfterSpawn (Insert button texts and icon)
  (Variables|Default|SetButton%20States (Utilities|Array|MakeArray "Desactivado" "Activado"))
  (Variables|Default|SetButton%20text "Mostrar controles")
  (Variables|Default|SetButton%20icon "/Game/FramearqTemplate/Blueprints/Pawn/VR/Oculus_controller/controller-icon.controller-icon")
  (bind _asbp_collab_v_player_controller (Utilities|Casting|CastToBP_Collab_V_PlayerController _returnvalue))
  (bind _returnvalue_2 (UserInterface|CreateWidget "/Game/FramearqTemplate/UMG/GameMenu/Settings_button.Settings_button_C" _returnvalue (Variables|Default|GetButton%20icon) (Variables|Default|GetButton%20text)))
  (bind _output_get (Variables|Default|SetButton%20Settings _returnvalue_2))
  (Class|HorizontalBox|AddChildtoHorizontalBox (Variables|/Game/FramearqTemplate/UMG/GameMenu/Contextual_Widget.Contextual_Widget_C|GetSecundary_Bar_Box (Variables|/Game/FramearqTemplate/Blueprints/PlayerController/BP_Collab_V_PlayerController.BP_Collab_V_PlayerController_C|GetContextualWidget _asbp_collab_v_player_controller)) _output_get)
  (CallFunction|CreateBindEvents)
  (CallFunction|SetButtonStatus))