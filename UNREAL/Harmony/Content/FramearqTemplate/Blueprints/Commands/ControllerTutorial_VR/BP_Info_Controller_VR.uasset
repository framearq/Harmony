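; BP_Info_Controller_VR is a VR menu command, "Info Controles", that shows or hides the controller tutorial.
; After the pawn spawns, it sets its icon and two Spanish option labels (show/hide controls), then creates a contextual button with those options.
; Each option is bound to an event that calls ShowTutorial or HideTutorial on BP_VRPawn, then restarts the menu on BP_BasePawn to reset the laser.
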(event Custom|Hide
  (params (id :type Integer) (Actor :type Actor%20Object%20Reference) (IsRightHand :type Boolean))
  (bind _asbp_vrpawn (Utilities|Casting|CastToBP_VRPawn (Game|Player|GetPlayerPawn 0)))
  (Default|HideTutorial _asbp_vrpawn)
  ;[1 1 1] restart laser
  (Default|RestartMenu (.AsBP%20Base%20Pawn (Utilities|Casting|CastToBP_BasePawn (Game|Player|GetPlayerPawn 0)))))

(event Custom|Show%20Plan
  (params (id :type Integer) (Actor :type Actor%20Object%20Reference) (IsRightHand :type Boolean))
  (bind _asbp_vrpawn (Utilities|Casting|CastToBP_VRPawn (Game|Player|GetPlayerPawn 0)))
  (Default|ShowTutorial _asbp_vrpawn)
  ;[1 1 1] restart laser
  (Default|RestartMenu (.AsBP%20Base%20Pawn (Utilities|Casting|CastToBP_BasePawn (Game|Player|GetPlayerPawn 0)))))

(event Custom|Bind_Options
  (bind _optionsbuttons (Variables|Default|GetOptionsButtons))
  (bind _optionsbuttons_2 (Variables|Default|GetOptionsButtons))
  (bind _output (Utilities|Array|Get(acopy) _optionsbuttons_2 1))
  (bind _output_2 (Utilities|Array|Get(acopy) _optionsbuttons))
  (Utilities|FlowControl|Sequence
    (:then_0
      (Variables|/Game/FramearqTemplate/UMG/GameMenu/Option_Button.Option_Button_C|SetWhenExecute _output_2 "NewEnumerator1")
      (EventDispatchers|BindEventtoExecute _output_2 (delegate Custom|Show%20Plan)))
    (:then_1
      (Variables|/Game/FramearqTemplate/UMG/GameMenu/Option_Button.Option_Button_C|SetWhenExecute _output "NewEnumerator1")
      (EventDispatchers|BindEventtoExecute _output (delegate Custom|Hide)))))

(event EventExecuteAfterSpawnPawn
  ;[0 1 0.1488] BeginPlayAfterSpawn
  (Variables|Default|SetIcon "/Game/FramearqTemplate/Blueprints/Pawn/VR/Oculus_controller/controller-icon.controller-icon")
  (Variables|Default|SetOptionsButtonNames (Utilities|Array|MakeArray "Mostrar Controles" "Ocultar Controles"))
  (Variables|Default|SetName "Info Controles")
  (CallFunction|SetBasePawn)
  (CallFunction|CreateContextualButon false true false)
  (CallFunction|BindOptions))