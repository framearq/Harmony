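; BP_Quit is the "Salir" contextual command, offering two options: return to the main menu or close the application.
; It configures its icon and labels after pawn spawn, then binds each option button to its handler.
; Both handlers destroy the network session first, then open the login menu level after a short delay or quit.
; The menu path first shows a VR splash loading screen or a UMG widget, depending on headset detection.
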(event Custom|Go%20to%20Main%20Menu
  (params (id :type Integer) (Actor :type Actor%20Object%20Reference) (IsRightHand :type Boolean))
  (CallFunction|ShowLoadindScreen)
  (|DestroySession (Game|GetPlayerController 0)
    (:then
      (Utilities|FlowControl|Delay 1.0)
      (Game|OpenLevel(byName) "Salon_LOGIN_Menu"))))

(event Custom|Close%20app
  (params (id :type Integer) (Actor :type Actor%20Object%20Reference) (IsRightHand :type Boolean))
  (|DestroySession (Game|GetPlayerController 0)
    (:then
      (Game|QuitGame 0 "Quit" false))))

(event Custom|Bind_Options
  (bind _optionsbuttons (Variables|Default|GetOptionsButtons))
  (bind _optionsbuttons_2 (Variables|Default|GetOptionsButtons))
  (bind _output (Utilities|Array|Get(acopy) _optionsbuttons_2 1))
  (bind _output_2 (Utilities|Array|Get(acopy) _optionsbuttons))
  (Utilities|FlowControl|Sequence
    (:then_0
      (Variables|/Game/FramearqTemplate/UMG/GameMenu/Option_Button.Option_Button_C|SetWhenExecute _output_2 "NewEnumerator1")
      (EventDispatchers|BindEventtoExecute _output_2 (delegate Custom|Go%20to%20Main%20Menu)))
    (:then_1
      (Variables|/Game/FramearqTemplate/UMG/GameMenu/Option_Button.Option_Button_C|SetWhenExecute _output "NewEnumerator1")
      (EventDispatchers|BindEventtoExecute _output (delegate Custom|Close%20app)))))

(event EventExecuteAfterSpawnPawn
  ;[0 1 0.1488] BeginPlayAfterSpawn
  (Variables|Default|SetIcon "/Game/FramearqTemplate/Blueprints/Commands/Quit/IconExit.IconExit")
  (Variables|Default|SetOptionsButtonNames (Utilities|Array|MakeArray "Menú principal" "Cerrar Aplicación"))
  (Variables|Default|SetName "Salir")
  (CallFunction|SetBasePawn)
  (CallFunction|CreateContextualButon false true false)
  (CallFunction|BindOptions)
  (bind _asbp_collaborative_viewer_game_instance (Utilities|Casting|CastToBP_CollaborativeViewer_GameInstance (Game|GetGameInstance)))
  (Variables|Default|SetGame%20Instance _asbp_collaborative_viewer_game_instance))

(fn ShowLoadindScreen
  (if (Math|Boolean|ORBoolean (Class|HeadMountedDisplayFunctionLibrary|IsHeadMountedDisplayEnabled) (and (Utilities|Enum|Equal(Enum) (Game|GetPlatformName) "Android") (Utilities|Name|NotEqual(Name) (Class|HeadMountedDisplayFunctionLibrary|GetHMDDeviceName) "None")) (== (Class|HeadMountedDisplayFunctionLibrary|GetHMDWornState) 1))
    (Class|XRLoadingScreenFunctionLibrary|AddLoadingScreenSplash "/Game/FramearqTemplate/UMG/Textures/pantalla-carga-VR.pantalla-carga-VR" "1.000000,0.000000,1.500000" "0, 0, 0" "(X=1.500000,Y=1.500000)" "0, 0, 0" true)
    (Class|XRLoadingScreenFunctionLibrary|ShowLoadingScreen)
    (else
      (bind _returnvalue (UserInterface|CreateWidget "/Game/FramearqTemplate/UMG/GameMenu/pantalla_carga.pantalla_carga_C"))
      (UserInterface|Viewport|AddtoViewport _returnvalue 0))))