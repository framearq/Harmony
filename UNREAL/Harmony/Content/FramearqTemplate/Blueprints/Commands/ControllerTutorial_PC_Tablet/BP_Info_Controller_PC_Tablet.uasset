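; Command Blueprint that adds an "Info Controles" button toggling the controls help overlay for PC and tablet.
; After the pawn spawns, it creates a Settings_button, with a touch icon on Android, in the Collab player controller's contextual secondary bar.
; On release, it adds or removes the controller's PcControllers widget, syncs the button's status and enabled state, then restarts the pawn's menu.
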(event Custom|Released%20Button
  (bind _button_settings (Variables|Default|GetButton%20Settings))
  (bind _button_settings_2 (Variables|Default|GetButton%20Settings))
  (bind _asbp_collab_v_player_controller (Utilities|Casting|CastToBP_Collab_V_PlayerController (Game|GetPlayerController 0)))
  (if (Widget|IsVisible (Variables|/Game/FramearqTemplate/Blueprints/PlayerController/BP_Collab_V_PlayerController.BP_Collab_V_PlayerController_C|GetPc_controllers _asbp_collab_v_player_controller))
    (Widget|RemovefromParent (Variables|/Game/FramearqTemplate/Blueprints/PlayerController/BP_Collab_V_PlayerController.BP_Collab_V_PlayerController_C|GetPc_controllers _asbp_collab_v_player_controller))
    (Variables|/Game/FramearqTemplate/UMG/GameMenu/Settings_button.Settings_button_C|SetButton_status _button_settings_2 (Utilities|Array|Get(acopy) (Variables|Default|GetButton%20States)))
    (Variables|/Game/FramearqTemplate/UMG/GameMenu/Settings_button.Settings_button_C|SetEnable%20state _button_settings false)
    (else
      (UserInterface|Viewport|AddtoViewport (Variables|/Game/FramearqTemplate/Blueprints/PlayerController/BP_Collab_V_PlayerController.BP_Collab_V_PlayerController_C|GetPc_controllers _asbp_collab_v_player_controller) 0)
      (Variables|/Game/FramearqTemplate/UMG/GameMenu/Settings_button.Settings_button_C|SetButton_status _button_settings_2 (Utilities|Array|Get(acopy) (Variables|Default|GetButton%20States) 1))
      (Variables|/Game/FramearqTemplate/UMG/GameMenu/Settings_button.Settings_button_C|SetEnable%20state _button_settings true)))
  (Default|RestartMenu (.AsBP%20Base%20Pawn (Utilities|Casting|CastToBP_BasePawn (Game|Player|GetPlayerPawn 0)))))

(event Custom|Bind%20Events
  (EventDispatchers|BindEventtoOnReleasedButton (Variables|Default|GetButton%20Settings) (delegate Custom|Released%20Button)))

(event EventExecuteAfterSpawnPawn
  (bind _returnvalue (Game|GetPlayerController 0))
  ;[0 1 0.1488] BeginPlayAfterSpawn (Insert button texts and icon)
  (Variables|Default|SetButton%20States (Utilities|Array|MakeArray "Desactivado" "Activado"))
  (Variables|Default|SetButton%20text "Info Controles")
  (if (Utilities|Enum|Equal(Enum) (Game|GetPlatformName) "Android")
    (Variables|Default|SetButton%20icon "/Game/FramearqTemplate/UMG/Textures/touch_app.touch_app")
    (else
      (Variables|Default|SetButton%20icon "/Game/FramearqTemplate/Blueprints/Commands/ControllerTutorial_PC_Tablet/controls-icon.controls-icon")))
  (bind _asbp_collab_v_player_controller (Utilities|Casting|CastToBP_Collab_V_PlayerController _returnvalue))
  (bind _returnvalue_2 (UserInterface|CreateWidget "/Game/FramearqTemplate/UMG/GameMenu/Settings_button.Settings_button_C" _returnvalue (Variables|Default|GetButton%20icon) (Variables|Default|GetButton%20text)))
  (bind _output_get (Variables|Default|SetButton%20Settings _returnvalue_2))
  (Class|HorizontalBox|AddChildtoHorizontalBox (Variables|/Game/FramearqTemplate/UMG/GameMenu/Contextual_Widget.Contextual_Widget_C|GetSecundary_Bar_Box (Variables|/Game/FramearqTemplate/Blueprints/PlayerController/BP_Collab_V_PlayerController.BP_Collab_V_PlayerController_C|GetContextualWidget _asbp_collab_v_player_controller)) _output_get)
  (CallFunction|BindEvents))