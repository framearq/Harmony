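; Day/night menu command that adds a contextual button with four time-of-day options to switch the level lighting.
; Options route through ROS-to-MTC event pairs that fade the camera (VR pawn on Android, camera manager elsewhere) and swap Day_Light and Night_Light streaming levels.
; The first option loads day; the other handlers all load night, and the fourth binds to the third button's index.
; An uncalled function shows a VR splash or widget loading screen.
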(event Custom|Go%20option%201
  (params (id :type Integer) (Actor :type Actor%20Object%20Reference) (IsRightHand :type Boolean))
  (Default|RestartMenu (.AsBP%20Base%20Pawn (Utilities|Casting|CastToBP_BasePawn (Game|Player|GetPlayerPawn 0))))
  (CallFunction|ToOption1ROS (Variables|Default|Getis%20Day?)))

(event Custom|go%20to%20option%204
  (params (id :type Integer) (Actor :type Actor%20Object%20Reference) (IsRightHand :type Boolean))
  (Default|RestartMenu (.AsBP%20Base%20Pawn (Utilities|Casting|CastToBP_BasePawn (Game|Player|GetPlayerPawn 0))))
  (CallFunction|ToOption2ROS (Variables|Default|Getis%20Day?)))

(event Custom|go%20to%20option%203
  (params (id :type Integer) (Actor :type Actor%20Object%20Reference) (IsRightHand :type Boolean))
  (Default|RestartMenu (.AsBP%20Base%20Pawn (Utilities|Casting|CastToBP_BasePawn (Game|Player|GetPlayerPawn 0))))
  (CallFunction|ToOption2ROS (Variables|Default|Getis%20Day?)))

(event Custom|to%20Option%203%20ROS
  (params (is%20Day? :type Boolean))
  (CallFunction|ToOption2MTC is%20Day?))

(event Custom|to%20Option%201%20MTC
  (params (is%20Day? :type Boolean))
  (bind _transitionspeed (Variables|Default|GetTransitionSpeed))
  ;[1 1 1] Fade Out
  (if (Utilities|Enum|Equal(Enum) (Game|GetPlatformName) "Android")
    (bind _asbp_vrpawn (Utilities|Casting|CastToBP_VRPawn (Game|Player|GetPlayerPawn 0)))
    (Default|CameraFadeStart _asbp_vrpawn)
    (else
      (CameraFades|StartCameraFade :self (Game|GetPlayerCameraManager 0) :ToAlpha 1.0 :Duration _transitionspeed :bShouldFadeAudio true :bHoldWhenFinished true)))
  (Utilities|FlowControl|Delay _transitionspeed)
  ;[1 1 1] Load Streaming Level
  (Game|UnloadStreamLevel(byName) "Night_Light" false)
  (Game|LoadStreamLevel(byName) "Day_Light" true)
  ;[1 1 1] Fade In
  (Utilities|FlowControl|Delay 2.0)
  (if (Utilities|Enum|Equal(Enum) (Game|GetPlatformName) "Android")
    (bind _asbp_vrpawn_2 (Utilities|Casting|CastToBP_VRPawn (Game|Player|GetPlayerPawn 0)))
    (Default|CameraFadeEnd _asbp_vrpawn_2)
    (else
      (CameraFades|StartCameraFade :self (Game|GetPlayerCameraManager 0) :FromAlpha 1.0 :Duration (Variables|Default|GetTransitionSpeed) :bShouldFadeAudio true))))

(event Custom|to%20Option%201%20ROS
  (params (is%20Day? :type Boolean))
  (CallFunction|ToOption1MTC is%20Day?))

(event Custom|to%20Option%202%20MTC
  (params (is%20Day? :type Boolean))
  (bind _transitionspeed (Variables|Default|GetTransitionSpeed))
  ;[1 1 1] Fade Out
  (if (Utilities|Enum|Equal(Enum) (Game|GetPlatformName) "Android")
    (bind _asbp_vrpawn (Utilities|Casting|CastToBP_VRPawn (Game|Player|GetPlayerPawn 0)))
    (Default|CameraFadeStart _asbp_vrpawn)
    (else
      (CameraFades|StartCameraFade :self (Game|GetPlayerCameraManager 0) :ToAlpha 1.0 :Duration _transitionspeed :bShouldFadeAudio true :bHoldWhenFinished true)))
  (Utilities|FlowControl|Delay _transitionspeed)
  ;[1 1 1] Load Streaming Level
  (Game|UnloadStreamLevel(byName) "Day_Light" false)
  (Game|LoadStreamLevel(byName) "Night_Light" true)
  ;[1 1 1] Fade In
  (Utilities|FlowControl|Delay 2.0)
  (if (Utilities|Enum|Equal(Enum) (Game|GetPlatformName) "Android")
    (bind _asbp_vrpawn_2 (Utilities|Casting|CastToBP_VRPawn (Game|Player|GetPlayerPawn 0)))
    (Default|CameraFadeEnd _asbp_vrpawn_2)
    (else
      (CameraFades|StartCameraFade :self (Game|GetPlayerCameraManager 0) :FromAlpha 1.0 :Duration (Variables|Default|GetTransitionSpeed) :bShouldFadeAudio true))))

(event Custom|to%20Option%204%20ROS
  (params (is%20Day? :type Boolean))
  (CallFunction|ToOption2MTC is%20Day?))

(event Custom|Go%20to%20option%202
  (params (id :type Integer) (Actor :type Actor%20Object%20Reference) (IsRightHand :type Boolean))
  (Default|RestartMenu (.AsBP%20Base%20Pawn (Utilities|Casting|CastToBP_BasePawn (Game|Player|GetPlayerPawn 0))))
  (CallFunction|ToOption2ROS (Variables|Default|Getis%20Day?)))

(event Custom|to%20Option%202%20ROS
  (params (is%20Day? :type Boolean))
  (CallFunction|ToOption2MTC is%20Day?))

(event Custom|Bind_Options
  (bind _optionsbuttons (Variables|Default|GetOptionsButtons))
  (bind _optionsbuttons_2 (Variables|Default|GetOptionsButtons))
  (bind _optionsbuttons_3 (Variables|Default|GetOptionsButtons))
  (bind _optionsbuttons_4 (Variables|Default|GetOptionsButtons))
  (bind _output (Utilities|Array|Get(acopy) _optionsbuttons_2 2))
  (bind _output_2 (Utilities|Array|Get(acopy) _optionsbuttons))
  (bind _output_3 (Utilities|Array|Get(acopy) _optionsbuttons_3 1))
  (bind _output_4 (Utilities|Array|Get(acopy) _optionsbuttons_4 2))
  (Utilities|FlowControl|Sequence
    (:then_0
      (Variables|/Game/FramearqTemplate/UMG/GameMenu/Option_Button.Option_Button_C|SetWhenExecute _output_2 "NewEnumerator1")
      (EventDispatchers|BindEventtoExecute _output_2 (delegate Custom|Go%20option%201)))
    (:then_1
      (Variables|/Game/FramearqTemplate/UMG/GameMenu/Option_Button.Option_Button_C|SetWhenExecute _output_3 "NewEnumerator1")
      (EventDispatchers|BindEventtoExecute _output_3 (delegate Custom|Go%20to%20option%202)))
    (:then_2
      (Variables|/Game/FramearqTemplate/UMG/GameMenu/Option_Button.Option_Button_C|SetWhenExecute _output_4 "NewEnumerator1")
      (EventDispatchers|BindEventtoExecute _output_4 (delegate Custom|go%20to%20option%203)))
    (:then_3
      (Variables|/Game/FramearqTemplate/UMG/GameMenu/Option_Button.Option_Button_C|SetWhenExecute _output "NewEnumerator1")
      (EventDispatchers|BindEventtoExecute _output (delegate Custom|go%20to%20option%204)))))

(event EventExecuteAfterSpawnPawn
  ;[0 1 0.1488] BeginPlayAfterSpawn
  (Variables|Default|SetIcon "/Game/FramearqTemplate/Blueprints/Commands/Day_Hours/day-night-icon.day-night-icon")
  (Variables|Default|SetOptionsButtonNames (Utilities|Array|MakeArray "10:00 " "14:00 " "20:00 " "23:00 "))
  (Variables|Default|SetName "Dia / Noche")
  (CallFunction|SetBasePawn)
  (CallFunction|CreateContextualButon false false false)
  (CallFunction|BindOptions))

(fn ShowLoadindScreen
  (if (Math|Boolean|ORBoolean (Class|HeadMountedDisplayFunctionLibrary|IsHeadMountedDisplayEnabled) (and (Utilities|Enum|Equal(Enum) (Game|GetPlatformName) "Android") (Utilities|Name|NotEqual(Name) (Class|HeadMountedDisplayFunctionLibrary|GetHMDDeviceName) "None")) (== (Class|HeadMountedDisplayFunctionLibrary|GetHMDWornState) 1))
    (Class|XRLoadingScreenFunctionLibrary|AddLoadingScreenSplash "/Game/FramearqTemplate/UMG/Textures/pantalla-carga-VR.pantalla-carga-VR" "1.000000,0.000000,1.500000" "0, 0, 0" "(X=1.500000,Y=1.500000)" "0, 0, 0" true)
    (Class|XRLoadingScreenFunctionLibrary|ShowLoadingScreen)
    (else
      (bind _returnvalue (UserInterface|CreateWidget "/Game/FramearqTemplate/UMG/GameMenu/pantalla_carga.pantalla_carga_C"))
      (UserInterface|Viewport|AddtoViewport _returnvalue 0))))

(fn OnRepIsDay?)