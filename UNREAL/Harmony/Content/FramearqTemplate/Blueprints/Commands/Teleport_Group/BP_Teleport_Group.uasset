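; Command blueprint that adds a "Mover en grupo" toggle button to the Collab Viewer contextual widget to switch group teleport on or off.
; Releasing the button flips the GameInstance TeleportGroup flag, updates the pawn and button, and shows or hides the VR controllers' group-teleport circle menu.
; The state is written to the SaveOptions save slot and restored on spawn, except clients always start with it off when a save exists.
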(event Custom|Create%20bind%20events
  ;[0 0.1794 1] Function
  (EventDispatchers|BindEventtoOnReleasedButton (Variables|Default|GetButton%20Settings) (delegate Custom|Released%20Button)))

(event Custom|Released%20Button
  (bind _button_settings (Variables|Default|GetButton%20Settings))
  (bind _button_settings_2 (Variables|Default|GetButton%20Settings))
  ;[0 0.1794 1] Function
  (bind _asbp_collaborative_viewer_game_instance (Utilities|Casting|CastToBP_CollaborativeViewer_GameInstance (Game|GetGameInstance)))
  (if (not (Variables|/Game/FramearqTemplate/Blueprints/GameInstance/BP_CollaborativeViewer_GameInstance.BP_CollaborativeViewer_GameInstance_C|Getteleport_group _asbp_collaborative_viewer_game_instance))
    (bind _asbp_base_pawn (Utilities|Casting|CastToBP_BasePawn (Game|Player|GetPlayerPawn 0)))
    (Variables|/Game/FramearqTemplate/Blueprints/Pawn/BP_BasePawn.BP_BasePawn_C|SetTeleport_group_Button_menu _asbp_base_pawn true)
    (Variables|/Game/FramearqTemplate/UMG/GameMenu/Settings_button.Settings_button_C|SetButton_status _button_settings_2 (Utilities|Array|Get(acopy) (Variables|Default|GetButton%20States) 1))
    (bind _asbp_collaborative_viewer_game_instance_2 (Utilities|Casting|CastToBP_CollaborativeViewer_GameInstance (Game|GetGameInstance)))
    (Variables|/Game/FramearqTemplate/Blueprints/GameInstance/BP_CollaborativeViewer_GameInstance.BP_CollaborativeViewer_GameInstance_C|Setteleport_group _asbp_collaborative_viewer_game_instance_2 true)
    (Variables|Default|SetTeleport_group_widget true)
    (bind _asbp_vrpawn (Utilities|Casting|CastToBP_VRPawn (Game|Player|GetPlayerPawn 0))
      (:then
        (Default|ShowHideTeleportGroupCircleMenu (Variables|/Game/FramearqTemplate/Blueprints/Pawn/VR/BP_VRPawn.BP_VRPawn_C|GetRightController _asbp_vrpawn) true))
      (:CastFailed
        _))
    (Development|PrintString "1")
    (Variables|/Game/FramearqTemplate/UMG/GameMenu/Settings_button.Settings_button_C|SetEnable%20state _button_settings true)
    (else
      (bind _asbp_base_pawn_2 (Utilities|Casting|CastToBP_BasePawn (Game|Player|GetPlayerPawn 0)))
      (Variables|/Game/FramearqTemplate/Blueprints/Pawn/BP_BasePawn.BP_BasePawn_C|SetTeleport_group_Button_menu _asbp_base_pawn_2 false)
      (Variables|/Game/FramearqTemplate/UMG/GameMenu/Settings_button.Settings_button_C|SetButton_status _button_settings_2 (Utilities|Array|Get(acopy) (Variables|Default|GetButton%20States)))
      (bind _asbp_collaborative_viewer_game_instance_3 (Utilities|Casting|CastToBP_CollaborativeViewer_GameInstance (Game|GetGameInstance)))
      (Variables|/Game/FramearqTemplate/Blueprints/GameInstance/BP_CollaborativeViewer_GameInstance.BP_CollaborativeViewer_GameInstance_C|Setteleport_group _asbp_collaborative_viewer_game_instance_3 false)
      (Variables|Default|SetTeleport_group_widget false)
      (bind _asbp_vrpawn_2 (Utilities|Casting|CastToBP_VRPawn (Game|Player|GetPlayerPawn 0))
        (:then
          (Default|ShowHideTeleportGroupCircleMenu (Variables|/Game/FramearqTemplate/Blueprints/Pawn/VR/BP_VRPawn.BP_VRPawn_C|GetRightController _asbp_vrpawn_2) false))
        (:CastFailed
          _))
      (Development|PrintString "0")
      (Variables|/Game/FramearqTemplate/UMG/GameMenu/Settings_button.Settings_button_C|SetEnable%20state _button_settings false)))
  ;[1 1 1] save mode
  (bind _returnvalue (SaveGame|DoesSaveGameExist (Variables|Default|GetSave_options)))
  (if _returnvalue
    (bind _returnvalue_2 (SaveGame|LoadGamefromSlot (Variables|Default|GetSave_options)))
    (Variables|Default|SetSave_game_mode _returnvalue_2)
    (else
      (bind _returnvalue_3 (SaveGame|CreateSaveGameObject "/Game/FramearqTemplate/Blueprints/SaveGame/BP_Save_player_options.BP_Save_player_options_C"))
      (Variables|Default|SetSave_game_mode _returnvalue_3)))
  (bind _asbp_save_player_options (Utilities|Casting|CastToBP_Save_player_options (Variables|Default|GetSave_game_mode)))
  (Variables|/Game/FramearqTemplate/Blueprints/SaveGame/BP_Save_player_options.BP_Save_player_options_C|SetTeleport_group _asbp_save_player_options (Variables|Default|GetTeleport_group_widget))
  (SaveGame|SaveGametoSlot (Variables|Default|GetSave_game_mode) (Variables|Default|GetSave_options)))

(event Custom|Set%20Button%20status
  (bind _button_settings (Variables|Default|GetButton%20Settings))
  (bind _button_settings_2 (Variables|Default|GetButton%20Settings))
  ;[1 1 1] Load
  (bind _returnvalue (SaveGame|DoesSaveGameExist (Variables|Default|GetSave_options)))
  (if _returnvalue
    (bind _returnvalue_2 (SaveGame|LoadGamefromSlot (Variables|Default|GetSave_options)))
    (bind _asbp_save_player_options (Utilities|Casting|CastToBP_Save_player_options _returnvalue_2))
    (bind _asbp_collaborative_viewer_game_instance (Utilities|Casting|CastToBP_CollaborativeViewer_GameInstance (Game|GetGameInstance)))
    ;[1 1 1] Si es cliente desactivamos el grupo siempre al inicio
    (if (Networking|IsServer)
      (Variables|/Game/FramearqTemplate/Blueprints/GameInstance/BP_CollaborativeViewer_GameInstance.BP_CollaborativeViewer_GameInstance_C|Setteleport_group _asbp_collaborative_viewer_game_instance (Variables|/Game/FramearqTemplate/Blueprints/SaveGame/BP_Save_player_options.BP_Save_player_options_C|GetTeleport_group _asbp_save_player_options))
      (else
        (Variables|/Game/FramearqTemplate/Blueprints/GameInstance/BP_CollaborativeViewer_GameInstance.BP_CollaborativeViewer_GameInstance_C|Setteleport_group _asbp_collaborative_viewer_game_instance false))))
  (bind _asbp_collaborative_viewer_game_instance_2 (Utilities|Casting|CastToBP_CollaborativeViewer_GameInstance (Game|GetGameInstance)))
  (if (Variables|/Game/FramearqTemplate/Blueprints/GameInstance/BP_CollaborativeViewer_GameInstance.BP_CollaborativeViewer_GameInstance_C|Getteleport_group _asbp_collaborative_viewer_game_instance_2)
    (Development|PrintString "Grupo activado")
    (Variables|/Game/FramearqTemplate/UMG/GameMenu/Settings_button.Settings_button_C|SetButton_status _button_settings (Utilities|Array|Get(acopy) (Variables|Default|GetButton%20States) 1))
    (Variables|Default|SetTeleport_group_widget true)
    (Variables|/Game/FramearqTemplate/UMG/GameMenu/Settings_button.Settings_button_C|SetEnable%20state _button_settings_2 true)
    (bind _asbp_base_pawn (Utilities|Casting|CastToBP_BasePawn (Game|Player|GetPlayerPawn 0)))
    (Variables|/Game/FramearqTemplate/Blueprints/Pawn/BP_BasePawn.BP_BasePawn_C|SetTeleport_group_Button_menu _asbp_base_pawn true)
    (else
      (Development|PrintString "Grupo desactivado")
      (Variables|/Game/FramearqTemplate/UMG/GameMenu/Settings_button.Settings_button_C|SetButton_status _button_settings (Utilities|Array|Get(acopy) (Variables|Default|GetButton%20States)))
      (Variables|Default|SetTeleport_group_widget false)
      (Variables|/Game/FramearqTemplate/UMG/GameMenu/Settings_button.Settings_button_C|SetEnable%20state _button_settings_2 false)
      (bind _asbp_base_pawn_2 (Utilities|Casting|CastToBP_BasePawn (Game|Player|GetPlayerPawn 0)))
      (Variables|/Game/FramearqTemplate/Blueprints/Pawn/BP_BasePawn.BP_BasePawn_C|SetTeleport_group_Button_menu _asbp_base_pawn_2 false))))

(event EventExecuteAfterSpawnPawn
  (bind _returnvalue (Game|GetPlayerController 0))
  ;[0 1 0.1488] BeginPlayAfterSpawn (Insert button texts and icon)
  (Variables|Default|SetButton%20States (Utilities|Array|MakeArray "Desactivado" "Activado"))
  (Variables|Default|SetButton%20text "Mover en grupo")
  (Variables|Default|SetButton%20icon "/Game/FramearqTemplate/UMG/Textures/teleport-group.teleport-group")
  (bind _asbp_collab_v_player_controller (Utilities|Casting|CastToBP_Collab_V_PlayerController _returnvalue))
  (bind _returnvalue_2 (UserInterface|CreateWidget "/Game/FramearqTemplate/UMG/GameMenu/Settings_button.Settings_button_C" _returnvalue (Variables|Default|GetButton%20icon) (Variables|Default|GetButton%20text)))
  (bind _output_get (Variables|Default|SetButton%20Settings _returnvalue_2))
  (Class|HorizontalBox|AddChildtoHorizontalBox (Variables|/Game/FramearqTemplate/UMG/GameMenu/Contextual_Widget.Contextual_Widget_C|GetSecundary_Bar_Box (Variables|/Game/FramearqTemplate/Blueprints/PlayerController/BP_Collab_V_PlayerController.BP_Collab_V_PlayerController_C|GetContextualWidget _asbp_collab_v_player_controller)) _output_get)
  (CallFunction|CreateBindEvents)
  (CallFunction|SetButtonStatus))