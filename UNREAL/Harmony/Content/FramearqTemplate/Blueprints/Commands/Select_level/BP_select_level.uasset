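; Framearq template command that adds a "Viviendas" contextual menu button, shown only on the server, for switching levels.
; After pawn spawn it reads LevelsData from the Collaborative Viewer GameInstance and builds the option buttons.
; Only the first level is listed and bound; handlers for further slots exist, but their binding code is unconnected.
; LoadLevel shows a VR splash or screen widget, then issues a servertravel command to the chosen map.
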(event Custom|A
  (params (id :type Integer) (Actor :type Actor%20Object%20Reference) (IsRightHand :type Boolean))
  (CallFunction|LoadLevel))

(event Custom|C
  (params (id :type Integer) (Actor :type Actor%20Object%20Reference) (IsRightHand :type Boolean))
  (CallFunction|LoadLevel 2))

(event Custom|CustomEvent_2
  (params (id :type Integer) (Actor :type Actor%20Object%20Reference) (IsRightHand :type Boolean))
  (CallFunction|LoadLevel 5))

(event Custom|CustomEvent
  (params (id :type Integer) (Actor :type Actor%20Object%20Reference) (IsRightHand :type Boolean))
  (CallFunction|LoadLevel 3))

(event Custom|B
  (params (id :type Integer) (Actor :type Actor%20Object%20Reference) (IsRightHand :type Boolean))
  (CallFunction|LoadLevel 1))

(event Custom|CustomEvent_3
  (params (id :type Integer) (Actor :type Actor%20Object%20Reference) (IsRightHand :type Boolean))
  (CallFunction|LoadLevel 6))

(event Custom|CustomEvent_1
  (params (id :type Integer) (Actor :type Actor%20Object%20Reference) (IsRightHand :type Boolean))
  (CallFunction|LoadLevel 4))

(event Custom|Bind_Options
  (bind _optionsbuttons (Variables|Default|GetOptionsButtons))
  (bind _output (Utilities|Array|Get(acopy) _optionsbuttons))
  (Utilities|FlowControl|Sequence
    (:then_0
      (Variables|/Game/FramearqTemplate/UMG/GameMenu/Option_Button.Option_Button_C|SetWhenExecute _output "NewEnumerator1")
      (EventDispatchers|BindEventtoExecute _output (delegate Custom|A)))))

(event EventExecuteAfterSpawnPawn
  ;[0 1 0.1488] BeginPlayAfterSpawn
  (bind _asbp_collaborative_viewer_game_instance (Utilities|Casting|CastToBP_CollaborativeViewer_GameInstance (Game|GetGameInstance)))
  (bind _output_get (Variables|Default|SetLevels%20Data (Variables|/Game/FramearqTemplate/Blueprints/GameInstance/BP_CollaborativeViewer_GameInstance.BP_CollaborativeViewer_GameInstance_C|GetLevels_data _asbp_collaborative_viewer_game_instance)))
  (Variables|Default|SetIcon "/Game/FramearqTemplate/Blueprints/Commands/Select_level/icono-vivienda.icono-vivienda")
  (Variables|Default|SetOptionsButtonNamesIcon (Utilities|Array|MakeArray (Utilities|Struct|MakeOption_button_names_icon (.level_name (Utilities|Array|Get(acopy) _output_get)) "/Game/FramearqTemplate/UMG/Textures/arrow_forward_ios.arrow_forward_ios")))
  (Variables|Default|SetName "Viviendas")
  (CallFunction|SetBasePawn)
  (CallFunction|CreateContextualButon false false (not (Networking|IsServer)))
  (CallFunction|BindOptions)
  (bind _asbp_collaborative_viewer_game_instance_2 (Utilities|Casting|CastToBP_CollaborativeViewer_GameInstance (Game|GetGameInstance)))
  (Variables|Default|SetGame%20Instance _asbp_collaborative_viewer_game_instance_2))

(fn ShowLoadindScreen
  (if (Math|Boolean|ORBoolean (Class|HeadMountedDisplayFunctionLibrary|IsHeadMountedDisplayEnabled) (and (Utilities|Enum|Equal(Enum) (Game|GetPlatformName) "Android") (Utilities|Name|NotEqual(Name) (Class|HeadMountedDisplayFunctionLibrary|GetHMDDeviceName) "None")) (== (Class|HeadMountedDisplayFunctionLibrary|GetHMDWornState) 1))
    (Class|XRLoadingScreenFunctionLibrary|AddLoadingScreenSplash "/Game/FramearqTemplate/UMG/Textures/pantalla-carga-VR.pantalla-carga-VR" "1.000000,0.000000,1.500000" "0, 0, 0" "(X=1.500000,Y=1.500000)" "0, 0, 0" true)
    (Class|XRLoadingScreenFunctionLibrary|ShowLoadingScreen)
    (else
      (bind _returnvalue (UserInterface|CreateWidget "/Game/FramearqTemplate/UMG/GameMenu/pantalla_carga.pantalla_carga_C"))
      (UserInterface|Viewport|AddtoViewport _returnvalue 0))))

(fn OnRepIsDay?)

(fn LoadLevel
  (params (Level%20Slot :type Integer))
  (CallFunction|ShowLoadindScreen)
  (Development|ExecuteConsoleCommand (Utilities|String|Append "servertravel /Game/Levels/" (Utilities|String|ToString(Name) (.level (Utilities|Array|Get(acopy) (Variables|Default|GetLevels%20Data) Level%20Slot)))) (Game|GetPlayerController 0)))