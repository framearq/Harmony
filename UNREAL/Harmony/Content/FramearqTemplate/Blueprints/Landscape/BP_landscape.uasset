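; Landscape backdrop actor that sets the image shown on a sphere mesh according to the current level and player position.
; Each tick, while a player character exists, it branches on the floor level name, with "Planta_cuarta" further split by the player's Y location.
; Set_Image creates a new dynamic material instance on the sphere at each call and writes the "Textura" parameter.
; An unconnected loop over TexturesByFloor is never run.
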(event EventBeginPlay)

(event EventTick
  (params (DeltaSeconds :type Float%20%28single-precision%29))
  (bind _returnvalue (Game|GetPlayerCharacter 0))
  (Utilities|IsValid _returnvalue
    (:Is%20Valid
      (bind _returnvalue_2 (Game|GetCurrentLevelName true))
      (if (not (Utilities|Enum|Equal(Enum) _returnvalue_2 "Planta_cuarta"))
        (if (Utilities|Enum|Equal(Enum) _returnvalue_2 "Planta_tercera")
          (CallFunction|SetImage)
          (else
            (CallFunction|SetImage)))
        (elif (<= (.y (Transformation|GetActorLocation _returnvalue)) -135.0)
          (CallFunction|SetImage)
          (else
            (CallFunction|SetImage)))))))

(fn ConstructionScript)

(fn SetImage
  (params (Image :type Texture%20Object%20Reference))
  (bind _returnvalue (Rendering|Material|CreateDynamicMaterialInstance (Variables|Default|GetSphere) 0 0 "None" :!class /Script/Engine.PrimitiveComponent))
  (Rendering|Material|SetTextureParameterValue _returnvalue "Textura" Image))