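; Game instance Blueprint for a collaborative viewer template that provides a loading screen suited to VR or flat-screen play.
; ShowLoadingScreen treats the session as VR when a headset is enabled, reported as worn, or named on Android.
; In VR it replaces any existing splash with a textured loading splash and shows it.
; Otherwise it creates the Pantalla_carga widget and adds it to the viewport.
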(fn ShowLoadingScreen
  (if (Math|Boolean|ORBoolean (Class|HeadMountedDisplayFunctionLibrary|IsHeadMountedDisplayEnabled) (and (Utilities|Enum|Equal(Enum) (Game|GetPlatformName) "Android") (Utilities|Name|NotEqual(Name) (Class|HeadMountedDisplayFunctionLibrary|GetHMDDeviceName) "None")) (== (Class|HeadMountedDisplayFunctionLibrary|GetHMDWornState) 1))
    (Class|XRLoadingScreenFunctionLibrary|AddLoadingScreenSplash "/Game/FramearqTemplate/UMG/Textures/pantalla-carga-VR.pantalla-carga-VR" "1.000000,0.000000,1.500000" "0, 0, 0" "(X=1.500000,Y=1.500000)" "0, 0, 0" true)
    (Class|XRLoadingScreenFunctionLibrary|ShowLoadingScreen)
    (else
      (bind _returnvalue (UserInterface|CreateWidget "/Game/FramearqTemplate/UMG/GameMenu/pantalla_carga.pantalla_carga_C"))
      (UserInterface|Viewport|AddtoViewport _returnvalue 0))))