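; Trigger volume actor that hides and shows the "Urbanizacion" streaming level as the player pawn enters and leaves its box.
; Begin overlap by the player's BP_BasePawn unloads the level, and end overlap loads it back visible, both without blocking.
; The HIdeStart flag also unloads the level on BeginPlay.
; Each change prints a colored on-screen debug message.
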(event OnComponentBeginOverlap(Box)
  (params (OverlappedComponent :type Primitive%20Component%20Object%20Reference) (OtherActor :type Actor%20Object%20Reference) (OtherComp :type Primitive%20Component%20Object%20Reference) (OtherBodyIndex :type Integer) (bFromSweep :type Boolean) (SweepResult :type Hit%20Result%20Structure%20%28by%20ref%29))
  (bind _asbp_base_pawn (Utilities|Casting|CastToBP_BasePawn (Game|Player|GetPlayerPawn 0)))
  (if (== _asbp_base_pawn OtherActor)
    (Game|UnloadStreamLevel(byName) "Urbanizacion" false)
    (Development|PrintString "Ocultado urbanizacion" true true "(R=1.000000,G=0.395417,B=0.000000,A=1.000000)" 5.0)))

(event OnComponentEndOverlap(Box)
  (params (OverlappedComponent :type Primitive%20Component%20Object%20Reference) (OtherActor :type Actor%20Object%20Reference) (OtherComp :type Primitive%20Component%20Object%20Reference) (OtherBodyIndex :type Integer))
  (bind _asbp_base_pawn (Utilities|Casting|CastToBP_BasePawn (Game|Player|GetPlayerPawn 0)))
  (if (== _asbp_base_pawn OtherActor)
    (Game|LoadStreamLevel(byName) "Urbanizacion" true)
    (Development|PrintString "Mostrado urbanizacion" true true "(R=0.927947,G=1.000000,B=0.000000,A=1.000000)" 5.0)))

(event EventBeginPlay
  (if (Variables|Default|GetHIde_Start)
    (Game|UnloadStreamLevel(byName) "Urbanizacion" false)
    (Development|PrintString "Ocultado urbanizacion" true true "(R=1.000000,G=0.395417,B=0.000000,A=1.000000)" 5.0)))

(fn ConstructionScript)