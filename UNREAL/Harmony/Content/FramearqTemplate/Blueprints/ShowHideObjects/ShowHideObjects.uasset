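; Trigger-box actor that shows or hides a list of Objects as the player's BP_BasePawn enters and leaves it.
; HideStart optionally hides every object at BeginPlay.
; MostarEntrar makes entry show and exit hide the objects; when false, the behavior is reversed.
; Colored Spanish debug prints report changes, though the exit print always reports "hidden" because its branch condition is fixed to true.
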(event OnComponentBeginOverlap(Box)
  (params (OverlappedComponent :type Primitive%20Component%20Object%20Reference) (OtherActor :type Actor%20Object%20Reference) (OtherComp :type Primitive%20Component%20Object%20Reference) (OtherBodyIndex :type Integer) (bFromSweep :type Boolean) (SweepResult :type Hit%20Result%20Structure%20%28by%20ref%29))
  (bind _mostar_entrar (Variables|Default|GetMostar_entrar))
  (bind _returnvalue (not _mostar_entrar))
  (bind _asbp_base_pawn (Utilities|Casting|CastToBP_BasePawn (Game|Player|GetPlayerPawn 0)))
  (if (== _asbp_base_pawn OtherActor)
    (for _array_element (Variables|Options|GetObjects)
      (Rendering|SetActorHiddenInGame _array_element _returnvalue)
      (if _returnvalue
        (Development|PrintString (Utilities|String|Append "Objeto Ocultado:" " " (Utilities|GetObjectName _array_element)) true true "(R=1.000000,G=0.000000,B=0.015653,A=1.000000)" 5.0)
        (else
          (Development|PrintString (Utilities|String|Append "Objeto mostrado:" " " (Utilities|GetObjectName _array_element)) true true "(R=0.110092,G=1.000000,B=0.000000,A=1.000000)" 5.0))))))

(event OnComponentEndOverlap(Box)
  (params (OverlappedComponent :type Primitive%20Component%20Object%20Reference) (OtherActor :type Actor%20Object%20Reference) (OtherComp :type Primitive%20Component%20Object%20Reference) (OtherBodyIndex :type Integer))
  (bind _asbp_base_pawn (Utilities|Casting|CastToBP_BasePawn (Game|Player|GetPlayerPawn 0)))
  (if (== _asbp_base_pawn OtherActor)
    (for _array_element (Variables|Options|GetObjects)
      (Rendering|SetActorHiddenInGame _array_element (Variables|Default|GetMostar_entrar))
      (if true
        (Development|PrintString (Utilities|String|Append "Objeto Ocultado:" " " (Utilities|GetObjectName _array_element)) true true "(R=1.000000,G=0.000000,B=0.015653,A=1.000000)" 5.0)
        (else
          (Development|PrintString (Utilities|String|Append "Objeto mostrado:" " " (Utilities|GetObjectName _array_element)) true true "(R=0.110092,G=1.000000,B=0.000000,A=1.000000)" 5.0))))))

(event EventBeginPlay
  (if (Variables|Default|GetHide_Start)
    (for _array_element (Variables|Options|GetObjects)
      (Rendering|SetActorHiddenInGame _array_element true)
      (Development|PrintString (Utilities|String|Append "Objeto Ocultado:" " " (Utilities|GetObjectName _array_element)) true true "(R=1.000000,G=0.000000,B=0.015653,A=1.000000)" 5.0))))

(fn ConstructionScript)